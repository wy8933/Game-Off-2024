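; BP_DimensionActor is an actor whose visibility follows the DimensionSeen and DimensionGone events of a BP_TwilightLantern.
; On BeginPlay it casts its owner to the lantern and binds both events, so it depends on that lantern being its owner.
; DimensionSeen unhides the actor and DimensionGone hides it, each printing an overlap debug message; BeginPlay sets no initial visibility.
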(event Custom|DimensionSeen_Event
  (Rendering|SetActorHiddenInGame false)
  (Development|PrintString "Overlapping"))

(event Custom|DimensionGone_Event
  (Rendering|SetActorHiddenInGame true)
  (Development|PrintString "No longer overlapping"))

(event EventBeginPlay
  (bind _returnvalue (Components|GetOwner))
  (bind _asbp_twilight_lantern (Utilities|Casting|CastToBP_TwilightLantern _returnvalue))
  (EventDispatchers|BindEventtoDimensionSeen _asbp_twilight_lantern (delegate Custom|DimensionSeen_Event))
  (bind _asbp_twilight_lantern_2 (Utilities|Casting|CastToBP_TwilightLantern _returnvalue))
  (EventDispatchers|BindEventtoDimensionGone _asbp_twilight_lantern_2 (delegate Custom|DimensionGone_Event)))

(event Collision|EventActorBeginOverlap
  (params (OtherActor :type Actor%20Object%20Reference)))

(event EventTick
  (params (DeltaSeconds :type Float%20%28single-precision%29)))

(fn ConstructionScript)