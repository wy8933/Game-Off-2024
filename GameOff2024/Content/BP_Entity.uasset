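; BP_Entity is an AI character that moves toward the first-person player when it sees them.
; PawnSensing's OnSeePawn filters for the player character, updates animation, then issues AIMoveTo to the location of the player's mesh.
; EntityAnimations plays assets directly on the mesh, starting a looping walk/run blend space once while in walking movement mode, otherwise a non-looping idle.
; Animation updates only on sightings, as Tick is empty.
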(event OnSeePawn(PawnSensing)
  (params (Pawn :type Pawn%20Object%20Reference))
  ;[1 1 1] Makes The Entity Follow the player if seen.
  (bind _asbp_first_person_character (Utilities|Casting|CastToBP_FirstPersonCharacter Pawn))
  (CallFunction|EntityAnimations)
  (AI|AIMoveTo self (Transformation|GetWorldLocation (Variables|/Script/Engine.Character|GetMesh _asbp_first_person_character)) 0 5.0 false))

(event EventBeginPlay)

(event Collision|EventActorBeginOverlap
  (params (OtherActor :type Actor%20Object%20Reference)))

(event EventTick
  (params (DeltaSeconds :type Float%20%28single-precision%29)))

(fn ConstructionScript)

(fn EntityAnimations
  (if (Pawn|Components|CharacterMovement|IsWalking (Variables|Character|GetCharacterMovement))
    (if (not (Variables|Default|GetIsEntityAnimRuningActive))
      (Variables|Default|SetIsEntityAnimRuningActive true)
      (Components|Animation|PlayAnimation (Variables|Character|GetMesh) "/Game/BookHeadMonster/Demo/Animations/BS_MM_WalkRun.BS_MM_WalkRun" true))
    (else
      (Variables|Default|SetIsEntityAnimRuningActive false)
      (Components|Animation|PlayAnimation (Variables|Character|GetMesh) "/Game/AnimationsMonstUE4pcs9/AnimationsUE4/Anim_Idle_Horror_Waiting_89_Motion.Anim_Idle_Horror_Waiting_89_Motion" false))))