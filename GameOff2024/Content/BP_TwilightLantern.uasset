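; Twilight lantern actor that acts as a lamp item the first-person player can show and hide.
; On BeginPlay it binds to the character's EquipLamp event, which toggles LampSelected and the actor's visibility.
; While visible, Tick snaps it to the player pawn's location and yaw with fixed pitch and a local offset, rather than attaching it.
; LampSelected reads inverted: true means hidden and not following.
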(event Custom|EquipLamp_Event
  (CallFunction|Hiding/ShowingLamp))

(event EventBeginPlay
  (bind _asbp_first_person_character (Utilities|Casting|CastToBP_FirstPersonCharacter (Game|GetPlayerCharacter 0)))
  (EventDispatchers|BindEventtoEquipLamp _asbp_first_person_character (delegate Custom|EquipLamp_Event)))

(event EventTick
  (params (DeltaSeconds :type Float%20%28single-precision%29))
  (if (not (Variables|Default|GetLampSelected))
    (CallFunction|LampItemUsage)))

(fn ConstructionScript)

(fn LampItemUsage
  (bind _returnvalue (Game|Player|GetPlayerPawn 0))
  (bind _returnvalue_2 (Transformation|GetActorRotation _returnvalue))
  (bind _output_get (Variables|Default|SetLampRotation (Math|Rotator|MakeRotator (.roll _returnvalue_2) -9e+01 (.yaw _returnvalue_2))))
  (Transformation|SetWorldTransform (Variables|Default|GetDefaultSceneRoot) (Math|Transform|MakeTransform (Transformation|GetActorLocation _returnvalue) _output_get "1.000000,1.000000,1.000000") false false)
  (Transformation|AddActorLocalOffset "-50.000000,35.000000,50.000000" false false))

(fn Hiding/ShowingLamp
  (if (Variables|Default|GetLampSelected)
    (Variables|Default|SetLampSelected false)
    (Rendering|SetActorHiddenInGame false)
    (else
      (Variables|Default|SetLampSelected true)
      (Rendering|SetActorHiddenInGame true))))