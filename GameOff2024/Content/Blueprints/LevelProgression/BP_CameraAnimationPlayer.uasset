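; Camera actor that plays spawn and death camera animations for the player.
; Each event blends the first player controller's view to this actor with a one-second cubic blend and starts its own timeline.
; The timeline's curve, scaled to degrees, drives the camera's relative roll, while pitch and yaw copy the player pawn's rotation on each update.
; Nothing in this graph returns the view to the pawn.
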(event Custom|PlayDeathCameraAnimation
  (bind _returnvalue (Game|Player|GetPlayerPawn 0))
  (bind _returnvalue_2 (Transformation|GetActorRotation _returnvalue))
  (Game|Player|SetViewTargetwithBlend (Game|GetPlayerController 0) self 1.0 "VTBlend_Cubic" 0.0 false)
  (bind _xrotation (Timeline|Timeline Play)
    (:Update
      (Transformation|SetRelativeRotation (Variables|Default|GetCamera) (Math|Rotator|MakeRotator (* _xrotation 9e+01) (.pitch _returnvalue_2) (.yaw _returnvalue_2)) false false))))

(event Custom|PlaySpawnCameraAnimation
  (bind _returnvalue (Game|Player|GetPlayerPawn 0))
  (bind _returnvalue_2 (Transformation|GetActorRotation _returnvalue))
  (Game|Player|SetViewTargetwithBlend (Game|GetPlayerController 0) self 1.0 "VTBlend_Cubic" 0.0 false)
  (bind _xrotation (Timeline|Timeline_0 Play)
    (:Update
      (Transformation|SetRelativeRotation (Variables|Default|GetCamera) (Math|Rotator|MakeRotator (* _xrotation 9e+01) (.pitch _returnvalue_2) (.yaw _returnvalue_2)) false false))))

(event EventBeginPlay)

(event Collision|EventActorBeginOverlap
  (params (OtherActor :type Actor%20Object%20Reference)))

(event EventTick
  (params (DeltaSeconds :type Float%20%28single-precision%29)))

(fn ConstructionScript)