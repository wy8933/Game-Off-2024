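; BP_Piano is an interactable piano puzzle that unlocks a linked door once the player has seen the music notes.
; Each interaction before success reports a wide-radius noise event and draws a matching debug sphere.
; It then reads the TimeTraveler pawn's HasSeenMusicNotes flag, playing a fail sound if false.
; If true, it plays the pass sound, unlocks the door, destroys its NavWall, blacks out the recording light and removes the widget.
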(event EventBeginPlay
  (|CallParentFunction) ; This node is disabled and will not be called.\nDrag off pins to build functionality.
)

(event Collision|EventActorBeginOverlap
  (params (OtherActor :type Actor%20Object%20Reference))
  (|CallParentFunction OtherActor) ; This node is disabled and will not be called.\nDrag off pins to build functionality.
)

(event EventTick
  (params (DeltaSeconds :type Float%20%28single-precision%29))
  (|CallParentFunction DeltaSeconds) ; This node is disabled and will not be called.\nDrag off pins to build functionality.
)

(event EventInteractBP
  (bind _returnvalue (Transformation|GetActorLocation))
  (bind _door (Variables|Default|GetDoor))
  (if (not (Variables|Default|GetPlayedSong))
    (Class|AISenseHearing|ReportNoiseEvent _returnvalue 1.0 self 4e+03 "None")
    (Rendering|Debug|DrawDebugSphere _returnvalue 4e+03 12 "(R=0.450763,G=0.000000,B=0.453125,A=1.000000)" 5.0)
    ;[1 1 1] Get HasSeenNotes bool from player
    (bind _asbp_time_traveler (Utilities|Casting|CastToBP_TimeTraveler (Game|Player|GetPlayerPawn 0)))
    (if (Variables|/Game/TimeTraval/BP_TimeTraveler.BP_TimeTraveler_C|GetbHasSeenMusicNotes _asbp_time_traveler)
      ;[1 1 1] True: play success track
      (Variables|Default|SetPlayedSong true)
      (Variables|/Game/Blueprints/Interactable/BP_Door.BP_Door_C|SetbLocked _door false)
      (Actor|DestroyActor (Variables|/Game/Blueprints/Interactable/BP_Door.BP_Door_C|GetNavWall _door))
      (Default|Unlock _door)
      (Rendering|Material|SetMaterial (Variables|Default|GetRecordingLight) 0 "/Game/Materials/M_Black.M_Black")
      (Components|DestroyComponent (Variables|Default|GetWidget))
      (Audio|PlaySoundatLocation "/Game/Audio_Game/Audio_Content/Music/PianoPassReal.PianoPassReal" (Transformation|GetActorLocation) "0, 0, 0" 1.0 1.0 0.0 0 0 0 0)
      (else
        ;[1 1 1] False: play failed track
        (Audio|PlaySoundatLocation "/Game/Audio_Game/Audio_Content/Music/PianoFail.PianoFail" (Transformation|GetActorLocation) "0, 0, 0" 1.0 1.0 0.0 0 0 0 0)))))

(fn ConstructionScript
  (|CallParentFunction))