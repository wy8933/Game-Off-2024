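; Interactable chair that blocks one or more doors until it is knocked aside.
; A one-time interaction plays a sound, reports a noise event and uses MoveComponentTo to slide and tilt the chair left or right according to MoveLeft.
; It then hides its widget and, for each referenced door, clears the lock, destroys its NavWall and calls Unlock.
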(event EventBeginPlay
  (|CallParentFunction) ; This node is disabled and will not be called.\nDrag off pins to build functionality.
)

(event Collision|EventActorBeginOverlap
  (params (OtherActor :type Actor%20Object%20Reference))
  (|CallParentFunction OtherActor) ; This node is disabled and will not be called.\nDrag off pins to build functionality.
)

(event EventTick
  (params (DeltaSeconds :type Float%20%28single-precision%29))
  (|CallParentFunction DeltaSeconds) ; This node is disabled and will not be called.\nDrag off pins to build functionality.
)

(event EventInteractBP
  (bind _chair (Variables|Default|GetChair))
  (bind _relativelocation (Variables|/Script/Engine.SceneComponent|GetRelativeLocation _chair))
  (bind _relativerotation (Variables|/Script/Engine.SceneComponent|GetRelativeRotation _chair))
  (if (not (Variables|Default|GetbHasMoved))
    (Variables|Default|SetbHasMoved true)
    (Audio|Components|Audio|Play (Variables|Default|GetMS_Interactable_Chair) 0.0)
    (Class|AISenseHearing|ReportNoiseEvent (Transformation|GetActorLocation) 1.0 self 1e+03 "None")
    (if (Variables|Default|GetMoveLeft)
      (Variables|Default|SetPushX 5e+02)
      (else
        (Variables|Default|SetPushX -5e+02)))
    (Components|MoveComponentTo _chair (Math|Vector|MakeVector (+ (.x _relativelocation) (Variables|Default|GetPushX)) (.y _relativelocation) (- (.z _relativelocation) 2e+01)) (Math|Rotator|MakeRotator (- (.roll _relativerotation) 27.5) (.pitch _relativerotation) (.yaw _relativerotation)) false false 0.5 false)
    (Rendering|SetVisibility (Variables|Default|GetWidget) false false)
    (for _array_element (Variables|Default|GetDoor)
      (Variables|/Game/Blueprints/Interactable/BP_Door.BP_Door_C|SetbLocked _array_element false)
      (Actor|DestroyActor (Variables|/Game/Blueprints/Interactable/BP_Door.BP_Door_C|GetNavWall _array_element))
      (Default|Unlock _array_element))))

(fn ConstructionScript
  (|CallParentFunction))