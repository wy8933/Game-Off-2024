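; BP_PressureValve is an interactable valve with a lever that toggles on and off, optionally as a puzzle piece.
; MoveLever smoothly pitches the Joint up or down by RotateValue according to IsOn, which flips after each interaction's move starts.
; BeginPlay moves the lever using the default RotateValue, then overrides that value for later swings.
; Puzzle valves also flip Correct, and on becoming correct ask the BP_ValveManager to check the valves.
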(event Custom|MoveLever
  (bind _joint (Variables|Default|GetJoint))
  (bind _joint_2 (Variables|Default|GetJoint))
  (bind _relativerotation (Variables|/Script/Engine.SceneComponent|GetRelativeRotation _joint))
  (bind _relativerotation_2 (Variables|/Script/Engine.SceneComponent|GetRelativeRotation _joint_2))
  (if (Variables|Default|GetbIsOn)
    (Components|MoveComponentTo _joint (Variables|/Script/Engine.SceneComponent|GetRelativeLocation _joint) (Math|Rotator|MakeRotator (.roll _relativerotation) (+ (.pitch _relativerotation) (Variables|Default|GetRotate%20Value)) (.yaw _relativerotation)) false false 0.4 false)
    (else
      (Components|MoveComponentTo _joint_2 (Variables|/Script/Engine.SceneComponent|GetRelativeLocation _joint_2) (Math|Rotator|MakeRotator (.roll _relativerotation_2) (- (.pitch _relativerotation_2) (Variables|Default|GetRotate%20Value)) (.yaw _relativerotation_2)) false false 0.4 false))))

(event EventBeginPlay
  (|CallParentFunction)
  (CallFunction|MoveLever)
  (Variables|Default|SetRotate%20Value 2.4e+02))

(event Collision|EventActorBeginOverlap
  (params (OtherActor :type Actor%20Object%20Reference))
  (|CallParentFunction OtherActor) ; This node is disabled and will not be called.\nDrag off pins to build functionality.
)

(event EventTick
  (params (DeltaSeconds :type Float%20%28single-precision%29))
  (|CallParentFunction DeltaSeconds) ; This node is disabled and will not be called.\nDrag off pins to build functionality.
)

(event EventInteractBP
  (CallFunction|MoveLever)
  (Variables|Default|SetbIsOn (not (Variables|Default|GetbIsOn)))
  (if (Variables|Default|GetbPuzzlePiece)
    (bind _output_get (Variables|Default|SetbCorrect (not (Variables|Default|GetbCorrect))))
    (if _output_get
      (bind _returnvalue (Actor|GetActorOfClass "/Game/Blueprints/BP_ValveManager.BP_ValveManager_C"))
      (Default|CheckValves _returnvalue))))

(fn ConstructionScript
  (|CallParentFunction))