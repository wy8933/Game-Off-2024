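; BP_KeyLock is an interactable lock that opens its linked doors when the player holds a key.
; On InteractBP, if BanquetLock is set, it casts the player pawn to BP_TimeTraveler and checks HasKey.
; With the key, it unlocks each Door entry, destroys their NavWalls and the Chains actors, then destroys itself.
; Interaction does nothing when BanquetLock is false.
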(event EventBeginPlay
  (|CallParentFunction) ; This node is disabled and will not be called.\nDrag off pins to build functionality.
)

(event Collision|EventActorBeginOverlap
  (params (OtherActor :type Actor%20Object%20Reference))
  (|CallParentFunction OtherActor) ; This node is disabled and will not be called.\nDrag off pins to build functionality.
)

(event EventTick
  (params (DeltaSeconds :type Float%20%28single-precision%29))
  (|CallParentFunction DeltaSeconds) ; This node is disabled and will not be called.\nDrag off pins to build functionality.
)

(event EventInteractBP
  (if (Variables|Default|GetbBanquetLock)
    (bind _asbp_time_traveler (Utilities|Casting|CastToBP_TimeTraveler (Game|Player|GetPlayerPawn 0)))
    (if (Variables|/Game/TimeTraval/BP_TimeTraveler.BP_TimeTraveler_C|GetbHasKey _asbp_time_traveler)
      (for _array_element (Variables|Default|GetDoor)
        (Variables|/Game/Blueprints/Interactable/BP_Door.BP_Door_C|SetbLocked _array_element false)
        (Actor|DestroyActor (Variables|/Game/Blueprints/Interactable/BP_Door.BP_Door_C|GetNavWall _array_element))
        (Default|Unlock _array_element))
      (for _array_element_2 (Variables|Default|GetChains)
        (Actor|DestroyActor _array_element_2))
      (Actor|DestroyActor))))

(fn ConstructionScript
  (|CallParentFunction))