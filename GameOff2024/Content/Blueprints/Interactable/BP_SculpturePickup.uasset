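; BP_SculpturePickup is an interactable collectible, one of five numbered sculptures that the time-traveler player can pick up.
; On interaction it plays an inventory foley sound, increments the player's sculpture count and sets the flag matching its Sculpture number.
; Each numbered pickup also raises BP_Entity's default chance to update zone, then destroys itself.
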(event EventBeginPlay)

(event Collision|EventActorBeginOverlap
  (params (OtherActor :type Actor%20Object%20Reference)))

(event EventTick
  (params (DeltaSeconds :type Float%20%28single-precision%29)))

(event EventInteractBP
  (Audio|PlaySoundatLocation "/Game/Audio_Game/Audio_Content/SFX/Interactable/MS_Inventory_Foley.MS_Inventory_Foley" (Transformation|GetActorLocation) "0, 0, 0" 1.0 1.0 0.0 0 0 0 0)
  (bind _asbp_time_traveler (Utilities|Casting|CastToBP_TimeTraveler (Game|Player|GetPlayerPawn 0)))
  (Variables|Default|SetPlayer _asbp_time_traveler)
  (Math|Integer|IncrementInt (Variables|/Game/TimeTraval/BP_TimeTraveler.BP_TimeTraveler_C|GetSculptures _asbp_time_traveler)
    (:%20%20
      (switch int (Variables|Default|GetSculpture)
        (:1
          (Variables|/Game/TimeTraval/BP_TimeTraveler.BP_TimeTraveler_C|SetGotSculpture1 (Variables|Default|GetPlayer) true))
        (:2
          (Variables|/Game/TimeTraval/BP_TimeTraveler.BP_TimeTraveler_C|SetGotSculpture2 (Variables|Default|GetPlayer) true))
        (:3
          (Variables|/Game/TimeTraval/BP_TimeTraveler.BP_TimeTraveler_C|SetGotSculpture3 (Variables|Default|GetPlayer) true))
        (:4
          (Variables|/Game/TimeTraval/BP_TimeTraveler.BP_TimeTraveler_C|SetGotSculpture4 (Variables|Default|GetPlayer) true))
        (:5
          (Variables|/Game/TimeTraval/BP_TimeTraveler.BP_TimeTraveler_C|SetGotSculpture5 (Variables|Default|GetPlayer) true)))
      (bind _returnvalue (Actor|GetActorOfClass "/Game/Blueprints/Enemy/BP_Entity.BP_Entity_C"))
      (Variables|/Game/Blueprints/Enemy/BP_Entity.BP_Entity_C|SetDefaultChanceToUpdateZone _returnvalue (+ (Variables|/Game/Blueprints/Enemy/BP_Entity.BP_Entity_C|GetDefaultChanceToUpdateZone _returnvalue) 5.0))
      (Actor|DestroyActor))))

(fn ConstructionScript)