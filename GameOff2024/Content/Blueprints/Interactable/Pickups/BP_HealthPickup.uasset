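; BP_HealthPickup is an interactable pickup that reacts when its InteractBP event fires.
; It plays the health interaction sound at its location, then casts the player pawn to BP_TimeTraveler to update the HUD notification and destroys itself.
; If the cast fails, the pickup is not destroyed.
; This graph contains no health change, and its BeginPlay, overlap and Tick events are disabled stubs.
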(event EventBeginPlay
  (|CallParentFunction) ; This node is disabled and will not be called.\nDrag off pins to build functionality.
)

(event Collision|EventActorBeginOverlap
  (params (OtherActor :type Actor%20Object%20Reference))
  (|CallParentFunction OtherActor) ; This node is disabled and will not be called.\nDrag off pins to build functionality.
)

(event EventTick
  (params (DeltaSeconds :type Float%20%28single-precision%29))
  (|CallParentFunction DeltaSeconds) ; This node is disabled and will not be called.\nDrag off pins to build functionality.
)

(event EventInteractBP
  (Audio|SpawnSoundatLocation "/Game/Audio_Game/Audio_Content/SFX/Interactable/MS_Interact_Health.MS_Interact_Health" (Transformation|GetActorLocation) "0, 0, 0" 1.0 1.0 0.0 0 0)
  (bind _asbp_time_traveler (Utilities|Casting|CastToBP_TimeTraveler (Game|Player|GetPlayerPawn 0)))
  (Default|UpdateHUDNotification _asbp_time_traveler)
  (Actor|DestroyActor))

(fn ConstructionScript
  (|CallParentFunction))