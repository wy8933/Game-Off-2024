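; Interactable bathroom door that the player or BP_Entity enemies swing open and closed.
; Inside/outside overlap boxes track each side, so ToggleDoor picks the 90-degree swing direction, inverted by Flipped, and animates it with MoveComponentTo.
; Enemies open it on proximity or toggle it on hit, suppressing player interaction while nearby.
; Locked doors start with trigger boxes disabled and NavWall hidden; Unlock re-enables boxes and updates the prompt.
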(event OnComponentBeginOverlap(InsideBox)
  (params (OverlappedComponent :type Primitive%20Component%20Object%20Reference) (OtherActor :type Actor%20Object%20Reference) (OtherComp :type Primitive%20Component%20Object%20Reference) (OtherBodyIndex :type Integer) (bFromSweep :type Boolean) (SweepResult :type Hit%20Result%20Structure%20%28by%20ref%29))
  (Utilities|Casting|CastToBP_TimeTraveler OtherActor)
  (Variables|Default|SetbPlayerInside true))

(event OnComponentBeginOverlap(OutsideBox)
  (params (OverlappedComponent :type Primitive%20Component%20Object%20Reference) (OtherActor :type Actor%20Object%20Reference) (OtherComp :type Primitive%20Component%20Object%20Reference) (OtherBodyIndex :type Integer) (bFromSweep :type Boolean) (SweepResult :type Hit%20Result%20Structure%20%28by%20ref%29))
  (Utilities|Casting|CastToBP_TimeTraveler OtherActor)
  (Variables|Default|SetbPlayerInside false))

(event OnComponentBeginOverlap(EnemyInsideBox)
  (params (OverlappedComponent :type Primitive%20Component%20Object%20Reference) (OtherActor :type Actor%20Object%20Reference) (OtherComp :type Primitive%20Component%20Object%20Reference) (OtherBodyIndex :type Integer) (bFromSweep :type Boolean) (SweepResult :type Hit%20Result%20Structure%20%28by%20ref%29))
  (Utilities|Casting|CastToBP_Entity OtherActor)
  (Variables|Default|SetbEnemyInside true))

(event OnComponentBeginOverlap(EnemyOutsideBox)
  (params (OverlappedComponent :type Primitive%20Component%20Object%20Reference) (OtherActor :type Actor%20Object%20Reference) (OtherComp :type Primitive%20Component%20Object%20Reference) (OtherBodyIndex :type Integer) (bFromSweep :type Boolean) (SweepResult :type Hit%20Result%20Structure%20%28by%20ref%29))
  (Utilities|Casting|CastToBP_Entity OtherActor)
  (Variables|Default|SetbEnemyInside false))

(event OnComponentBeginOverlap(EnemyBox)
  (params (OverlappedComponent :type Primitive%20Component%20Object%20Reference) (OtherActor :type Actor%20Object%20Reference) (OtherComp :type Primitive%20Component%20Object%20Reference) (OtherBodyIndex :type Integer) (bFromSweep :type Boolean) (SweepResult :type Hit%20Result%20Structure%20%28by%20ref%29))
  (Utilities|Casting|CastToBP_Entity OtherActor)
  (Variables|Default|SetbCanInteract false)
  (Rendering|SetVisibility (Variables|Default|GetWidget) false false)
  (if (not (Variables|Default|GetbDoorOpen))
    (if (Utilities|Operators|EqualEqual (Variables|/Script/Engine.SceneComponent|GetRelativeRotation (Variables|Default|GetDoor)) (Variables|Default|GetDefaultRotation) 0.5)
      (CallFunction|EnemyOpen))))

(event OnComponentEndOverlap(EnemyBox)
  (params (OverlappedComponent :type Primitive%20Component%20Object%20Reference) (OtherActor :type Actor%20Object%20Reference) (OtherComp :type Primitive%20Component%20Object%20Reference) (OtherBodyIndex :type Integer))
  (Utilities|Casting|CastToBP_Entity OtherActor)
  (Variables|Default|SetbCanInteract true)
  (Rendering|SetVisibility (Variables|Default|GetWidget) true false))

(event OnComponentHit(Door)
  (params (HitComponent :type Primitive%20Component%20Object%20Reference) (OtherActor :type Actor%20Object%20Reference) (OtherComp :type Primitive%20Component%20Object%20Reference) (NormalImpulse :type Vector :default "0, 0, 0") (Hit :type Hit%20Result%20Structure%20%28by%20ref%29))
  (Utilities|Casting|CastToBP_Entity OtherActor)
  (Variables|Default|SetbBoolToCheck (Variables|Default|GetbEnemyInside))
  (CallFunction|ToggleDoor))

(event Custom|PlayerOpen
  (Variables|Default|SetbBoolToCheck (Variables|Default|GetbPlayerInside))
  (CallFunction|ToggleDoor))

(event Custom|EnemyOpen
  (Variables|Default|SetbBoolToCheck (Variables|Default|GetbEnemyInside))
  (CallFunction|ToggleDoor))

(event Custom|ToggleDoor
  (bind _bflipped (Variables|Default|GetbFlipped))
  (bind _defaultrotation (Variables|Default|GetDefaultRotation))
  (Collision|SetCollisionEnabled (Variables|Default|GetDoor) "NoCollision")
  (if (Variables|Default|GetbDoorOpen)
    (Audio|Components|Audio|Play (Variables|Default|GetMS_Door_Close_Preset) 0.0)
    (Utilities|FlowControl|Sequence
      (:then_0
        (goto _label_4 Stop))
      (:then_1
        (Components|MoveComponentTo (Variables|Default|GetDoor) (Variables|Default|GetDefaultLocation) (Variables|Default|GetDefaultRotation) true true 0.5 false :!label _label)
        (Variables|Default|SetbDoorOpen false)
        (Collision|SetCollisionEnabled (Variables|Default|GetDoor) "QueryAndPhysics")))
    (else
      (Audio|Components|Audio|Play (Variables|Default|GetMS_Door_Open) 0.0)
      (Utilities|FlowControl|Sequence
        (:then_0
          (goto _label Stop))
        (:then_1
          (Collision|SetCollisionEnabled (Variables|Default|GetDoor) "NoCollision")
          (if (Variables|Default|GetbBoolToCheck)
            (if _bflipped
              (Variables|Default|SetOpenZRotation (- (.yaw _defaultrotation) 9e+01) :!label _label_2)
              (else
                (Variables|Default|SetOpenZRotation (+ (.yaw _defaultrotation) 9e+01) :!label _label_3)))
            (elif _bflipped
              (goto _label_3)
              (else
                (goto _label_2))))
          (Components|MoveComponentTo (Variables|Default|GetDoor) (Variables|Default|GetDefaultLocation) (Math|Rotator|MakeRotator (.roll _defaultrotation) (.pitch _defaultrotation) (Variables|Default|GetOpenZRotation)) true true 0.5 false :!label _label_4)
          (Variables|Default|SetbDoorOpen true)
          (Collision|SetCollisionEnabled (Variables|Default|GetDoor) "QueryAndPhysics"))))))

(event Custom|Unlock
  (Collision|SetCollisionEnabled (Variables|Default|GetEnemyBox) "QueryAndPhysics")
  (Collision|SetCollisionEnabled (Variables|Default|GetEnemyOutsideBox) "QueryAndPhysics")
  (Collision|SetCollisionEnabled (Variables|Default|GetEnemyInsideBox) "QueryAndPhysics")
  (Collision|SetCollisionEnabled (Variables|Default|GetOutsideBox) "QueryAndPhysics")
  (Collision|SetCollisionEnabled (Variables|Default|GetInsideBox) "QueryAndPhysics")
  (Variables|Default|SetInteractionType "Open")
  (Class|InteractableActor|SetWidgetPromptText))

(event EventBeginPlay
  (bind _door (Variables|Default|GetDoor))
  (bind _navwall (Variables|Default|GetNavWall))
  (|CallParentFunction)
  (Variables|Default|SetDefaultLocation (Variables|/Script/Engine.SceneComponent|GetRelativeLocation _door))
  (Variables|Default|SetDefaultRotation (Variables|/Script/Engine.SceneComponent|GetRelativeRotation _door))
  (if (Variables|Default|GetbLocked)
    (Collision|SetCollisionEnabled (Variables|Default|GetEnemyBox) "NoCollision")
    (Collision|SetCollisionEnabled (Variables|Default|GetEnemyOutsideBox) "NoCollision")
    (Collision|SetCollisionEnabled (Variables|Default|GetEnemyInsideBox) "NoCollision")
    (Collision|SetCollisionEnabled (Variables|Default|GetOutsideBox) "NoCollision")
    (Collision|SetCollisionEnabled (Variables|Default|GetInsideBox) "NoCollision")
    (Utilities|IsValid _navwall
      (:Is%20Valid
        (Rendering|SetActorHiddenInGame _navwall true)))))

(event Collision|EventActorBeginOverlap
  (params (OtherActor :type Actor%20Object%20Reference))
  (|CallParentFunction OtherActor) ; This node is disabled and will not be called.\nDrag off pins to build functionality.
)

(event EventTick
  (params (DeltaSeconds :type Float%20%28single-precision%29))
  (|CallParentFunction DeltaSeconds) ; This node is disabled and will not be called.\nDrag off pins to build functionality.
)

(event EventInteractBP
  (if (and (Variables|Default|GetbCanInteract) (not (Variables|Default|GetbLocked)))
    (CallFunction|PlayerOpen)))

(fn ConstructionScript
  (|CallParentFunction))