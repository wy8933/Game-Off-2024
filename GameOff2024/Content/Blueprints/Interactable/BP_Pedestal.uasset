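; BP_Pedestal is an interactable pedestal tied to one of five sculptures through its Sculpture index.
; On InteractBP it casts the player pawn to BP_TimeTraveler, stores it, and switches on the index to check the matching GotSculpture flag.
; The branches lead to no actions, so interacting has no visible effect yet, and the other events are empty stubs.
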(event EventBeginPlay)

(event Collision|EventActorBeginOverlap
  (params (OtherActor :type Actor%20Object%20Reference)))

(event EventTick
  (params (DeltaSeconds :type Float%20%28single-precision%29)))

(event EventInteractBP
  (bind _asbp_time_traveler (Utilities|Casting|CastToBP_TimeTraveler (Game|Player|GetPlayerPawn 0)))
  (Variables|Default|SetPlayer _asbp_time_traveler)
  (switch int (Variables|Default|GetSculpture)
    (:1
      (if (Variables|/Game/TimeTraval/BP_TimeTraveler.BP_TimeTraveler_C|GetGotSculpture1 (Variables|Default|GetPlayer))
        _))
    (:2
      (if (Variables|/Game/TimeTraval/BP_TimeTraveler.BP_TimeTraveler_C|GetGotSculpture2 (Variables|Default|GetPlayer))
        _))
    (:3
      (if (Variables|/Game/TimeTraval/BP_TimeTraveler.BP_TimeTraveler_C|GetGotSculpture3 (Variables|Default|GetPlayer))
        _))
    (:4
      (if (Variables|/Game/TimeTraval/BP_TimeTraveler.BP_TimeTraveler_C|GetGotSculpture4 (Variables|Default|GetPlayer))
        _))
    (:5
      (if (Variables|/Game/TimeTraval/BP_TimeTraveler.BP_TimeTraveler_C|GetGotSculpture5 (Variables|Default|GetPlayer))
        _))))

(fn ConstructionScript)