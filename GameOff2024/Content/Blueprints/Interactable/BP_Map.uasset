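; BP_Map is an interactable map pickup that gives the player either the ground floor or second floor map.
; On InteractBP, the SecondFloorMap flag selects which ownership boolean to set on the player's BP_TimeTraveler pawn.
; It also applies the matching floor material to that pawn's Map, then destroys itself.
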(event EventBeginPlay)

(event Collision|EventActorBeginOverlap
  (params (OtherActor :type Actor%20Object%20Reference)))

(event EventTick
  (params (DeltaSeconds :type Float%20%28single-precision%29)))

(event EventInteractBP
  (if (Variables|Default|GetSecondFloorMap)
    (bind _asbp_time_traveler (Utilities|Casting|CastToBP_TimeTraveler (Game|Player|GetPlayerPawn 0)))
    (Variables|/Game/TimeTraval/BP_TimeTraveler.BP_TimeTraveler_C|SetbHasSecondFloorMap _asbp_time_traveler true)
    (Rendering|Material|SetMaterial (Variables|/Game/TimeTraval/BP_TimeTraveler.BP_TimeTraveler_C|GetMap _asbp_time_traveler) 0 "/Game/Art/Textures/M_SecondFloorMap.M_SecondFloorMap")
    (else
      (bind _asbp_time_traveler_2 (Utilities|Casting|CastToBP_TimeTraveler (Game|Player|GetPlayerPawn 0)))
      (Variables|/Game/TimeTraval/BP_TimeTraveler.BP_TimeTraveler_C|SetbHasGroundFloorMap _asbp_time_traveler_2 true)
      (Rendering|Material|SetMaterial (Variables|/Game/TimeTraval/BP_TimeTraveler.BP_TimeTraveler_C|GetMap _asbp_time_traveler_2) 0 "/Game/Art/Textures/M_GroundFloorMap.M_GroundFloorMap")))
  (Actor|DestroyActor))

(fn ConstructionScript)