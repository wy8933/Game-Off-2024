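; BP_ItemSpawnManager is a manager actor that randomly thins placed health, bottle and ammo pickups when play begins.
; For each array in turn, it loops a DeleteItems function that destroys a random element and removes it until the count is no longer above that type's target quantity.
; Each loop deletes before checking, so every array loses at least one item.
; The manager destroys itself once all three are trimmed.
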(event EventBeginPlay
  (bind _ammopickuparray (Variables|Default|GetAmmoPickupArray))
  (bind _healthpickuparray (Variables|Default|GetHealthPickupArray))
  (bind _bottlepickuparray (Variables|Default|GetBottlePickupArray))
  (CallFunction|DeleteItems _healthpickuparray :!label _label)
  (if (> (Utilities|Array|Length _healthpickuparray) (Variables|Default|GetHealthPickupQuantity))
    (goto _label)
    (else
      (CallFunction|DeleteItems _bottlepickuparray :!label _label_2)
      (if (> (Utilities|Array|Length _bottlepickuparray) (Variables|Default|GetBottlePickupQuantity))
        (goto _label_2)
        (else
          (CallFunction|DeleteItems _ammopickuparray :!label _label_3)
          (if (> (Utilities|Array|Length _ammopickuparray) (Variables|Default|GetAmmoPickupQuantity))
            (goto _label_3)
            (else
              (Actor|DestroyActor))))))))

(event Collision|EventActorBeginOverlap
  (params (OtherActor :type Actor%20Object%20Reference)))

(event EventTick
  (params (DeltaSeconds :type Float%20%28single-precision%29)))

(fn ConstructionScript)

(fn DeleteItems
  (params (TargetArray :type Array%20of%20Interactable%20Actor%20Object%20References))
  (Variables|Default|SetRandomInt (Math|Random|RandomInteger (Utilities|Array|Length TargetArray)))
  (Actor|DestroyActor (Utilities|Array|Get(acopy) TargetArray (Variables|Default|GetRandomInt)))
  (Utilities|Array|RemoveIndex TargetArray (Variables|Default|GetRandomInt)))