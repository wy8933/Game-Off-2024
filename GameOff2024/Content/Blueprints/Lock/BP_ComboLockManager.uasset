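; Combination lock manager actor that unlocks a door once the password is correct.
; On BeginPlay it registers four BP_ComboLockPart child actors through AddLock and sets itself as their owner.
; CheckUnlock tests IsPasswordCorrect, then unlocks the Door and destroys its NavWall.
; It then tilts and shifts the Latch, and after a short delay destroys both the latch and itself.
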(event Custom|CheckUnlock
  (bind _latch (Variables|Default|GetLatch))
  (bind _latch_2 (Variables|Default|GetLatch))
  (bind _door (Variables|Default|GetDoor))
  (bind _returnvalue (Transformation|GetActorLocation _latch_2))
  (bind _returnvalue_2 (Transformation|GetActorRotation _latch))
  (if (Variables|Default|GetbIsPasswordCorrect)
    (Variables|/Game/Blueprints/Interactable/BP_Door.BP_Door_C|SetbLocked _door false)
    (Actor|DestroyActor (Variables|/Game/Blueprints/Interactable/BP_Door.BP_Door_C|GetNavWall _door))
    (Default|Unlock _door)
    (Transformation|SetActorRotation _latch (Math|Rotator|MakeRotator (.roll _returnvalue_2) (+ (.pitch _returnvalue_2) 6e+01) (.yaw _returnvalue_2)))
    (Transformation|SetActorLocation _latch_2 (Math|Vector|MakeVector (- (.x _returnvalue) 15.0) (.y _returnvalue) (.z _returnvalue)) false false)
    (Utilities|FlowControl|Delay 1.0)
    (Actor|DestroyActor (Variables|Default|GetLatch))
    (Actor|DestroyActor)))

(event EventBeginPlay
  (bind _self self)
  (bind _bp_combolockpart1 (Variables|Default|GetBP_ComboLockPart1))
  (bind _bp_combolockpart4 (Variables|Default|GetBP_ComboLockPart4))
  (bind _bp_combolockpart2 (Variables|Default|GetBP_ComboLockPart2))
  (bind _bp_combolockpart3 (Variables|Default|GetBP_ComboLockPart3))
  (bind _childactor (Variables|/Script/Engine.ChildActorComponent|GetChildActor _bp_combolockpart1))
  (bind _childactor_2 (Variables|/Script/Engine.ChildActorComponent|GetChildActor _bp_combolockpart4))
  (bind _childactor_3 (Variables|/Script/Engine.ChildActorComponent|GetChildActor _bp_combolockpart2))
  (bind _childactor_4 (Variables|/Script/Engine.ChildActorComponent|GetChildActor _bp_combolockpart3))
  ;[1 1 1] Add the lock to the manager
  (bind _asbp_combo_lock_part (Utilities|Casting|CastToBP_ComboLockPart _childactor))
  (Class|ComboLockManager|AddLock _asbp_combo_lock_part)
  (Actor|SetOwner _childactor _self)
  (bind _asbp_combo_lock_part_2 (Utilities|Casting|CastToBP_ComboLockPart _childactor_3))
  (Class|ComboLockManager|AddLock _asbp_combo_lock_part_2)
  (Actor|SetOwner _childactor_3 _self)
  (bind _asbp_combo_lock_part_3 (Utilities|Casting|CastToBP_ComboLockPart _childactor_4))
  (Class|ComboLockManager|AddLock _asbp_combo_lock_part_3)
  (Actor|SetOwner _childactor_4 _self)
  (bind _asbp_combo_lock_part_4 (Utilities|Casting|CastToBP_ComboLockPart _childactor_2))
  (Class|ComboLockManager|AddLock _asbp_combo_lock_part_4)
  (Actor|SetOwner _childactor_2 _self))

(event EventTick
  (params (DeltaSeconds :type Float%20%28single-precision%29)))

(fn ConstructionScript)