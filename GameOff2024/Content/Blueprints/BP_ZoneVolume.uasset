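; BP_ZoneVolume is a box trigger volume that records which zone the time traveler is in.
; When a BP_TimeTraveler begins overlapping the box, it sets that character's CurrentZone to the volume's Zone value.
; If its Enemy reference is valid, zone 6 also unlocks the enemy's access to zone 1, and zone 8 unlocks access to zone 8.
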(event OnComponentBeginOverlap(Box)
  (params (OverlappedComponent :type Primitive%20Component%20Object%20Reference) (OtherActor :type Actor%20Object%20Reference) (OtherComp :type Primitive%20Component%20Object%20Reference) (OtherBodyIndex :type Integer) (bFromSweep :type Boolean) (SweepResult :type Hit%20Result%20Structure%20%28by%20ref%29))
  (bind _zone (Variables|Default|GetZone))
  (bind _enemy (Variables|Default|GetEnemy))
  (bind _enemy_2 (Variables|Default|GetEnemy))
  (bind _asbp_time_traveler (Utilities|Casting|CastToBP_TimeTraveler OtherActor))
  (Variables|/Game/TimeTraval/BP_TimeTraveler.BP_TimeTraveler_C|SetCurrentZone _asbp_time_traveler (Variables|Default|GetZone))
  (Utilities|IsValid (Variables|Default|GetEnemy)
    (:Is%20Valid
      (if (== _zone 6)
        (if (not (Variables|/Game/BP_Entity.BP_Entity_C|GetCanEnterZone1 _enemy_2))
          (Variables|/Game/BP_Entity.BP_Entity_C|SetCanEnterZone1 _enemy true))
        (elif (== _zone 8)
          (if (not (Variables|/Game/BP_Entity.BP_Entity_C|GetCanEnterZone8 _enemy_2))
            (Variables|/Game/BP_Entity.BP_Entity_C|SetCanEnterZone8 _enemy true)))))))

(event EventBeginPlay)

(event Collision|EventActorBeginOverlap
  (params (OtherActor :type Actor%20Object%20Reference)))

(event EventTick
  (params (DeltaSeconds :type Float%20%28single-precision%29)))

(fn ConstructionScript)