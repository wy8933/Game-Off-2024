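; Enemy AI character that patrols, hunts and attacks the time-traveling player, draining health on reaching them.
; PawnSensing sight fills a detection meter, scaled by crouch or sprint, leading to a chase or last-known-location search; noises trigger investigation.
; Tick drives random patrols within zone point arrays, which can switch to the player's zone by weighted chance or on chase.
; The player's PauseTime flag gates sensing, chasing and patrol.
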(event OnHearNoise(PawnSensing)
  (params (Instigator :type Pawn%20Object%20Reference) (Location :type Vector%20%28by%20ref%29 :default "0, 0, 0") (Volume :type Float%20%28single-precision%29))
  ;[1 1 1] Audio Detection
  (Development|PrintString "Heard")
  (if (not (Variables|/Game/TimeTraval/BP_TimeTraveler.BP_TimeTraveler_C|GetPauseTime (stale EventBeginPlay _asbp_time_traveler)))
    (if (not (or (Variables|AI|GetIsEntityChasingPlayer?) (Variables|AI|GetIsEntityInvestigating)))
      (Variables|AI|SetIsEntityInvestigating true)
      (AI|AIMoveTo self Location Instigator 5.0 false
        (:OnSuccess
          (Variables|AI|SetIsEntityInvestigating false))))))

(event OnSeePawn(PawnSensing)
  (params (Pawn :type Pawn%20Object%20Reference))
  ;[1 1 1] Visual Detection
  (if (not (Variables|/Game/TimeTraval/BP_TimeTraveler.BP_TimeTraveler_C|GetPauseTime (stale EventBeginPlay _asbp_time_traveler)))
    (Utilities|FlowControl|Sequence
      (:then_0
        (Utilities|FlowControl|Sequence
          (:then_0
            (Utilities|FlowControl|DoOnce false :!label _label
              (:Completed
                (CallFunction|StartDetection))))
          (:then_1
            (CallFunction|UpdateLastKnownLocation)
            (if (not (Variables|AI|GetIsEntityChasingPlayer?))
              (if (Variables|Detection|GetDetectingPlayer)
                (if (>= (Variables|Detection|GetDetection) 1.0)
                  (CallFunction|Chase)
                  (else
                    (CallFunction|SetDetectionRate)
                    (CallFunction|DetectPlayer))))))))
      (:then_1
        (Utilities|FlowControl|RetriggerableDelay 0.5)
        (CallFunction|StopDetection)
        (Utilities|FlowControl|Sequence
          (:then_0
            (goto _label Reset))
          (:then_1
            (if (> (Variables|Detection|GetDetection) 0.5)
              (Variables|Detection|SetDetection 0.0)
              (CallFunction|CheckLastKnownLocation))))))))

(event Custom|Chase
  ;[1 1 1] Chase
  (if (not (Variables|/Game/TimeTraval/BP_TimeTraveler.BP_TimeTraveler_C|GetPauseTime (stale EventBeginPlay _asbp_time_traveler)))
    (CallFunction|InitiateChase)
    ;;[1 1 1] Managed Animations
    (Utilities|ChasingAnimations)
    (CallFunction|UpdateZone)
    (AI|AIMoveTo self "0, 0, 0" (Variables|Default|GetPlayer) 5.0 false
      (:OnSuccess
        (CallFunction|AttackPlayer))
      (:OnFail
        ;[1 1 1] Return to patrol
        (Variables|AI|SetIsEntityChasingPlayer? false)
        (Variables|Default|SetIsEntityAnimRuningActive false)
        (bind _returnvalue (CallFunction|GetRandomTargetPoint (Variables|Arrays|GetPatrolingLocations)))
        (Variables|AI|SetCurrentLocation _returnvalue)))))

(event Custom|CheckLastKnownLocation
  (bind _lastknownlocation (Variables|Default|GetLastKnownLocation))
  ;[1 1 1] Check Last Known Location
  (if (not (Variables|/Game/TimeTraval/BP_TimeTraveler.BP_TimeTraveler_C|GetPauseTime (stale EventBeginPlay _asbp_time_traveler)))
    (Rendering|Debug|DrawDebugSphere _lastknownlocation 1e+02 12 "(R=1.000000,G=1.000000,B=1.000000,A=1.000000)" 1e+01)
    (bind _movementresult (AI|AIMoveTo self _lastknownlocation 0 5.0 false)
      (:OnSuccess
        _)
      (:OnFail
        (Development|PrintString (Utilities|String|EnumtoString _movementresult))))
    (Variables|AI|SetIsEntityChasingPlayer? false)
    (Variables|Default|SetIsEntityAnimRuningActive false)
    (Development|PrintString "Return to patrol")
    (bind _returnvalue (CallFunction|GetRandomTargetPoint (Variables|Arrays|GetPatrolingLocations)))
    (Variables|AI|SetCurrentLocation _returnvalue)
    (Variables|Default|SetVisibilityTimerSet false)))

(event EventBeginPlay
  ;[1 1 1] Initialize
  (bind _asbp_time_traveler (Utilities|Casting|CastToBP_TimeTraveler (Game|Player|GetPlayerPawn 0)))
  (Variables|Default|SetPlayer _asbp_time_traveler)
  (Utilities|Array|Clear (Variables|Arrays|GetPatrolingLocations))
  (CallFunction|AddtoPatrolArray (Variables|Arrays|GetZoneArray3))
  (bind _returnvalue (CallFunction|GetRandomTargetPoint (Variables|Arrays|GetPatrolingLocations)))
  (Variables|AI|SetCurrentLocation _returnvalue))

(event EventTick
  (params (DeltaSeconds :type Float%20%28single-precision%29))
  (bind _isentitychasingplayer_ (Variables|AI|GetIsEntityChasingPlayer?))
  (bind _patrolinglocations (Variables|Arrays|GetPatrolingLocations))
  ;[1 1 1] Handles The Patroling
  (if (Variables|/Game/TimeTraval/BP_TimeTraveler.BP_TimeTraveler_C|GetPauseTime (stale EventBeginPlay _asbp_time_traveler))
    (if (Variables|AI|GetIsEntityRunning?)
      (if (not (Variables|Default|GetChaseSoundPlaying))
        (bind _returnvalue (Audio|SpawnSound2D "/Game/Audios/MonsterSounds/Level1IntenseTake2.Level1IntenseTake2" 1.0 1.0 0.0 0))
        (Variables|Default|SetChaseSoundPlaying true)
        (Components|Activation|SetActive _returnvalue _isentitychasingplayer_ false))
      (elif (not _isentitychasingplayer_)
        (Variables|AI|SetIsEntityRunning? true)
        (Variables|/Script/Engine.CharacterMovementComponent|SetMaxWalkSpeed (Variables|Character|GetCharacterMovement) (Variables|Default|GetWalkSpeed))
        (if (Utilities|Array|IsValidIndex _patrolinglocations (Variables|AI|GetCurrentLocation))
          (AI|AIMoveTo self "0, 0, 0" (Utilities|Array|Get(acopy) _patrolinglocations (Variables|AI|GetCurrentLocation)) 5.0 false
            (:OnSuccess
              ;;[1 1 1] Cicles through the Array
              (Utilities|FlowControl|Delay (Math|Random|RandomFloatinRange 2.0 5.0))
              (CallFunction|CyclingPatrolingArray (Variables|Arrays|GetPatrolingLocations))
              (Variables|AI|SetIsEntityRunning? false))
            (:OnFail
              (Development|PrintString "Patrol Failed")
              (Variables|AI|SetIsEntityRunning? false))))))))

(fn ConstructionScript)

(fn EntityAnimations
  (if (not (Variables|Default|GetIsEntityAnimRuningActive))
    (Variables|Default|SetIsEntityAnimRuningActive true)
    (Components|Animation|PlayAnimation (Variables|Character|GetMesh) "/Game/AnimationsMonstUE4pcs9/AnimationsUE4/Anim_Walking_Looking_150_Motion.Anim_Walking_Looking_150_Motion" true)))

(fn CyclingPatrolingArray
  (params (TargetArray :type Array%20of%20Target%20Point%20Object%20References))
  (bind _returnvalue (Math|Random|RandomFloatinRange 0.0 1e+02))
  ;[1 1 1] Check if currently in player's zone
  (if (== (Variables|/Game/TimeTraval/BP_TimeTraveler.BP_TimeTraveler_C|GetCurrentZone (Variables|Default|GetPlayer)) (Variables|AI|GetCurrentZone))
    (Development|PrintString "Current Zone")
    ;[1 1 1] Select random target point and set current location
    (bind _returnvalue_2 (CallFunction|GetRandomTargetPoint TargetArray :!label _label))
    (Variables|AI|SetCurrentLocation _returnvalue_2)
    (Development|PrintString "Selected new random point")
    (else
      ;[1 1 1] Check if AI can enter safe zone if player is inside safe zone
      (if (and (== (Variables|/Game/TimeTraval/BP_TimeTraveler.BP_TimeTraveler_C|GetCurrentZone (Variables|Default|GetPlayer)) 1) (not (Variables|AI|GetCanEnterZone1)))
        (Development|PrintString "Player in safe zone, cannot enter")
        (goto _label)
        (else
          (Development|PrintString (Utilities|String|ToString(Float) _returnvalue))
          ;[1 1 1] Chance to update zone. Low = new zone, high = stay in old zone
          (if (<= _returnvalue (Variables|AI|GetChanceToUpdateZone))
            (Development|PrintString "Increasing chance")
            ;[1 1 1] Increase zone update chance if it's not already over 90%
            (if (<= (Variables|AI|GetChanceToUpdateZone) 9e+01)
              (Variables|AI|SetChanceToUpdateZone (+ (Variables|AI|GetChanceToUpdateZone) 1e+01))
              (goto _label)
              (else
                (goto _label)))
            (else
              (Development|PrintString "Updating zone")
              (CallFunction|UpdateZone))))))))

(fn GetRandomTargetPoint
  (params (TargetArray :type Array%20of%20Target%20Point%20Object%20References))
  (return (Math|Random|RandomInteger (Utilities|Array|Length TargetArray))))

(fn AddtoPatrolArray
  (params (Array :type Array%20of%20Target%20Point%20Object%20References))
  (for _array_element Array
    (Utilities|Array|AddUnique (Variables|Arrays|GetPatrolingLocations) _array_element))
  (return))

(fn UpdateZone
  ;[1 1 1] Clear patrol array and update zone to follow player
  (Variables|AI|SetChanceToUpdateZone 2e+01)
  (Utilities|Array|Clear (Variables|Arrays|GetPatrolingLocations))
  (bind _output_get (Variables|AI|SetCurrentZone (Variables|/Game/TimeTraval/BP_TimeTraveler.BP_TimeTraveler_C|GetCurrentZone (Variables|Default|GetPlayer))))
  ;[1 1 1] Add new zone array to the patrol array
  (switch int _output_get
    (:1
      (CallFunction|AddtoPatrolArray (Variables|Arrays|GetZoneArray1)))
    (:2
      (CallFunction|AddtoPatrolArray (Variables|Arrays|GetZoneArray2)))
    (:3
      (CallFunction|AddtoPatrolArray (Variables|Arrays|GetZoneArray3)))
    (:4
      (CallFunction|AddtoPatrolArray (Variables|Arrays|GetZoneArray4)))
    (:5
      (CallFunction|AddtoPatrolArray (Variables|Arrays|GetZoneArray5)))
    (:6
      (CallFunction|AddtoPatrolArray (Variables|Arrays|GetZoneArray6)))
    (:7
      (CallFunction|AddtoPatrolArray (Variables|Arrays|GetZoneArray7)))
    (:8
      (CallFunction|AddtoPatrolArray (Variables|Arrays|GetZoneArray8))))
  ;[1 1 1] Select random target point and set current location
  (bind _returnvalue (CallFunction|GetRandomTargetPoint (Variables|Arrays|GetPatrolingLocations)))
  (Variables|AI|SetCurrentLocation _returnvalue))

(fn AttackPlayer
  (Variables|AI|SetIsEntityChasingPlayer? false)
  (Variables|Default|SetIsEntityAnimRuningActive false)
  (Components|Animation|PlayAnimation (Variables|Character|GetMesh) "/Game/AnimationsMonstUE4pcs9/AnimationsUE4/Anim_EatsPrey_110_Motion.Anim_EatsPrey_110_Motion" false)
  ;[1 1 1] Drains Player's Health
  (bind _asbp_time_traveler (Utilities|Casting|CastToBP_TimeTraveler (Game|GetPlayerCharacter 0)))
  (Variables|/Game/TimeTraval/BP_TimeTraveler.BP_TimeTraveler_C|SetHealth _asbp_time_traveler (Math|Float|Clamp(Float) (- (Variables|/Game/TimeTraval/BP_TimeTraveler.BP_TimeTraveler_C|GetHealth _asbp_time_traveler) 35.0) 0.0 1e+02)))

(fn InitiateChase
  (Variables|AI|SetIsEntityChasingPlayer? true)
  (Variables|AI|SetIsEntityRunning? false)
  (Variables|/Script/Engine.CharacterMovementComponent|SetMaxWalkSpeed (Variables|Character|GetCharacterMovement) (Variables|Default|GetChaseSpeed)))

(fn StartDetection
  (Variables|Detection|SetDetectingPlayer true))

(fn DetectPlayer
  (Variables|Detection|SetDetection (+ (Variables|Detection|GetDetection) (Variables|Detection|GetDetectionRate))))

(fn StopDetection
  (Variables|Detection|SetDetectingPlayer false)
  (Development|PrintString "stop detection"))

(fn SetDetectionRate
  (bind _player (Variables|Default|GetPlayer))
  (bind _charactermovement (Variables|/Script/Engine.Character|GetCharacterMovement _player))
  (if (AI|Components|NavMovement|IsCrouching _charactermovement)
    (Variables|Detection|SetDetectionRate 0.1)
    (elif (== (Variables|/Script/Engine.CharacterMovementComponent|GetMaxWalkSpeed _charactermovement) (Variables|/Script/GameOff2024.GameOff2024Character|GetMaxSprintSpeed _player))
      (Variables|Detection|SetDetectionRate 0.35)
      (else
        (Variables|Detection|SetDetectionRate 0.15)))))

(fn UpdateLastKnownLocation
  (bind _player (Variables|Default|GetPlayer))
  (bind _returnvalue (Transformation|GetActorLocation _player))
  (bind _outhit (Collision|LineTraceByChannel (Transformation|GetActorLocation _player) (Math|Vector|MakeVector (.x _returnvalue) (.y _returnvalue) (- (.z _returnvalue) 1e+03)) "TraceTypeQuery1" false (Utilities|Array|MakeArray _player) "ForDuration"))
  (Variables|Default|SetLastKnownLocation (.Location (Collision|BreakHitResult _outhit))))