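; Stalking monster enemy that patrols eight zones, hunts the time-traveler player and melee-attacks on reaching them.
; Patrols drift toward the player's zone with escalating probability, respecting a safe zone.
; Sight builds detection by player movement state, noises trigger investigation, and full detection or proximity starts a chase.
; Hitbox delegates make headshots force flight to another zone; body and limb hits compare fixed damage to HP without subtracting it.
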(event OnTargetPerceptionUpdated(AIPerception)
  (params (Actor :type Actor%20Object%20Reference) (Stimulus :type AI%20Stimulus%20Structure))
  (bind (_age _expirationage _strength _stimuluslocation _receiverlocation _tag _bsuccessfullysensed) (Utilities|Struct|BreakAIStimulus Stimulus))
  ;[1 1 1] Audio Detection
  (if _bsuccessfullysensed
    (Utilities|FlowControl|Sequence
      (:then_0
        (Development|PrintString "Heard")
        (if (not (or (Variables|AI|GetIsEntityChasingPlayer?) (Variables|AI|GetIsEntityInvestigating)))
          (Variables|AI|SetIsEntityInvestigating true)
          (AI|AIMoveTo self _stimuluslocation 0 5.0 false
            (:OnSuccess
              _)
            (:OnFail
              _))
          (Utilities|FlowControl|Delay (Math|Random|RandomFloatinRange 2.0 5.0))
          (if (not (Variables|AI|GetIsEntityChasingPlayer?))
            (CallFunction|ReturntoPatrol))))
      (:then_1
        ;[0.3506 0.208 1] Play Alert
        (Utilities|FlowControl|DoOnce false
          (:Completed
            (Audio|Components|Audio|Play (Variables|Default|GetMS_Monster_Alert) 0.0)))))))

(event OnSeePawn(PawnSensing)
  (params (Pawn :type Pawn%20Object%20Reference))
  ;[1 1 1] Visual Detection
  (Utilities|FlowControl|Sequence
    (:then_0
      (Utilities|FlowControl|Sequence
        (:then_0
          (Utilities|FlowControl|DoOnce false :!label _label
            (:Completed
              (CallFunction|StartDetection))))
        (:then_1
          (CallFunction|UpdateLastKnownLocation)
          (if (not (Variables|AI|GetIsEntityChasingPlayer?))
            (if (Variables|Detection|GetDetectingPlayer)
              (if (>= (Variables|Detection|GetDetection) 1.0)
                (CallFunction|Chase)
                (else
                  (CallFunction|SetDetectionRate)
                  (CallFunction|DetectPlayer))))))))
    (:then_1
      (Utilities|FlowControl|RetriggerableDelay 0.5)
      (CallFunction|StopDetection)
      (Utilities|FlowControl|Sequence
        (:then_0
          (goto _label Reset))
        (:then_1
          (if (> (Variables|Detection|GetDetection) 0.5)
            (Variables|Detection|SetDetection 0.0)
            (CallFunction|CheckLastKnownLocation)))))
    (:then_2
      (Development|PrintString "Hello"))))

(event OnComponentBeginOverlap(DetectionSphere)
  (params (OverlappedComponent :type Primitive%20Component%20Object%20Reference) (OtherActor :type Actor%20Object%20Reference) (OtherComp :type Primitive%20Component%20Object%20Reference) (OtherBodyIndex :type Integer) (bFromSweep :type Boolean) (SweepResult :type Hit%20Result%20Structure%20%28by%20ref%29))
  (bind _asbp_time_traveler (Utilities|Casting|CastToBP_TimeTraveler OtherActor))
  (Development|PrintString "Auto Chase")
  (if (== (Components|SkeletalMesh|GetSkeletalMeshAsset (Variables|/Script/Engine.Character|GetMesh _asbp_time_traveler)) OtherComp)
    (CallFunction|Chase)))

(event OnComponentBeginOverlap(AttackCollision)
  (params (OverlappedComponent :type Primitive%20Component%20Object%20Reference) (OtherActor :type Actor%20Object%20Reference) (OtherComp :type Primitive%20Component%20Object%20Reference) (OtherBodyIndex :type Integer) (bFromSweep :type Boolean) (SweepResult :type Hit%20Result%20Structure%20%28by%20ref%29))
  (Utilities|Casting|CastToBP_TimeTraveler OtherActor)
  (CallFunction|DamagePlayer))

(event Custom|Return%20To%20Patrol
  ;[1 1 1] Return to patrol
  (Variables|AI|SetIsEntityChasingPlayer? false)
  (Variables|AI|SetIsEntityRunning? false)
  (Variables|AI|SetIsEntityInvestigating false)
  (bind _returnvalue (CallFunction|GetRandomTargetPoint (Variables|Arrays|GetPatrolingLocations)))
  (Variables|AI|SetCurrentLocation _returnvalue))

(event Custom|Headshot
  (params (impactPoint :type Vector))
  ;[1 1 1] Hitbox Events for getting shot
  (CallFunction|BloodParticle impactPoint)
  (if (> (Variables|Default|GetHP) 0)
    (CallFunction|Flee)))

(event Custom|PlayAlertSound
  ;[0.3506 0.208 1] Play Alert
  (Utilities|FlowControl|DoOnce false
    (:Completed
      (Audio|Components|Audio|Play (Variables|Default|GetMS_Monster_Alert) 0.0))))

(event Custom|Chase
  ;[1 1 1] Chase
  (if (not (Variables|AI|GetIsEntityChasingPlayer?))
    (CallFunction|InitiateChase)
    (CallFunction|UpdateZone (Variables|/Game/TimeTraval/BP_TimeTraveler.BP_TimeTraveler_C|GetCurrentZone (Variables|Default|GetPlayer)))
    (AI|AIMoveTo self "0, 0, 0" (Variables|Default|GetPlayer) 5.0 false
      (:OnSuccess
        (Development|PrintString "Attack")
        (CallFunction|AttackPlayer))
      (:OnFail
        (CallFunction|ReturntoPatrol)))))

(event Custom|CheckLastKnownLocation
  (bind _lastknownlocation (Variables|Default|GetLastKnownLocation))
  ;[1 1 1] Check Last Known Location
  (Rendering|Debug|DrawDebugSphere _lastknownlocation 5e+02 12 "(R=1.000000,G=1.000000,B=1.000000,A=1.000000)" 1e+01)
  (Components|Movement|StopMovementImmediately (Variables|Character|GetCharacterMovement))
  (bind (_randomlocation _returnvalue) (Class|NavigationSystemV1|GetRandomLocationinNavigableRadius _lastknownlocation 5e+02 0 0))
  (Development|PrintText (Utilities|Text|ToText(Boolean) _returnvalue))
  (bind _movementresult (AI|AIMoveTo self _randomlocation 0 5.0 false)
    (:OnSuccess
      _)
    (:OnFail
      (Development|PrintString (Utilities|String|EnumtoString _movementresult))))
  (Utilities|FlowControl|Delay (Math|Random|RandomFloatinRange 2.0 5.0))
  (CallFunction|ReturntoPatrol))

(event Custom|Bodyshot
  (params (impactPoint :type Vector))
  ;[1 1 1] Hitbox Events for getting shot
  (CallFunction|BloodParticle impactPoint)
  (if (> (Variables|Default|GetHP) 0)
    (if (<= (- (Variables|Default|GetHP) 5) 0)
      (CallFunction|Flee))))

(event Custom|Limbshot
  (params (impactPoint :type Vector))
  ;[1 1 1] Hitbox Events for getting shot
  (CallFunction|BloodParticle impactPoint)
  (if (> (Variables|Default|GetHP) 0)
    (if (<= (- (Variables|Default|GetHP) 3) 0)
      (CallFunction|Flee))))

(event Custom|Flee
  (bind _patrolinglocations (Variables|Arrays|GetPatrolingLocations))
  ;[1 1 1] Flee
  (Audio|Components|Audio|Play (Variables|Default|GetMS_Monster_Hurt) 0.0)
  (Animation|Montage|MontagePlay (Variables|Default|GetAnimInstance) "/Game/Blueprints/Enemy/Animations/Montages/AM_EntityCrawl.AM_EntityCrawl" 1.0 "MontageLength" 0.0 true)
  (Variables|AI|SetIsEntityChasingPlayer? false)
  (Variables|AI|SetIsEntityRunning? true)
  (Variables|AI|SetIsEntityInvestigating false)
  (Variables|Default|SetHP 0)
  (Development|PrintString "Flee")
  (bind _output_get (Variables|Default|SetNewZone (Math|Random|RandomIntegerinRange 1 8) :!label _label))
  (if (== _output_get (Variables|AI|GetCurrentZone))
    (goto _label)
    (else
      (bind _output_get_2 (Variables|AI|SetCurrentZone (Variables|Default|GetNewZone)))
      (CallFunction|UpdateZone _output_get_2)
      (if (Utilities|Array|IsValidIndex _patrolinglocations (Variables|AI|GetCurrentLocation))
        (AI|AIMoveTo self "0, 0, 0" (Utilities|Array|Get(acopy) _patrolinglocations (Variables|AI|GetCurrentLocation)) 5.0 false
          (:OnSuccess
            (Variables|Default|SetHP (Variables|Default|GetMaxHP))
            (Utilities|FlowControl|Delay (Math|Random|RandomFloatinRange 2.0 5.0))
            (if (not (or (Variables|AI|GetIsEntityChasingPlayer?) (Variables|AI|GetIsEntityInvestigating)))
              (Variables|AI|SetIsEntityRunning? false)
              (CallFunction|CyclingPatrolingArray (Variables|Arrays|GetPatrolingLocations))
              (Animation|Montage|MontageStop (Variables|Default|GetAnimInstance) 0.0 "/Game/Blueprints/Enemy/Animations/Montages/AM_EntityCrawl.AM_EntityCrawl" :!label _label_2)))
          (:OnFail
            (Development|PrintString "Failed to flee")
            (Variables|AI|SetIsEntityRunning? false)
            (Variables|Default|SetHP (Variables|Default|GetMaxHP))
            (goto _label_2)))))))

(event Custom|AttackEnd
  (Variables|AI|SetIsEntityChasingPlayer? false)
  (Variables|AI|SetIsEntityInvestigating false)
  (Variables|/Script/Engine.PrimitiveComponent|SetbGenerateOverlapEvents (Variables|Default|GetAttackCollision) false))

(event Custom|BloodParticle
  (params (Location :type Vector))
  (Niagara|SpawnSystematLocation "/Game/Art/Particles/Character/BloodSplatter/PS_BloodSplatter.PS_BloodSplatter" Location))

(event Custom|Reset_Alert_Sound
  ;[0.3506 0.208 1] Play Alert
  (Development|PrintString "ALERT RESET")
  (Utilities|FlowControl|DoOnce false) ; enters at Reset
)

(event EventBeginPlay
  ;[1 1 1] Initialize
  (bind _asbp_time_traveler (Utilities|Casting|CastToBP_TimeTraveler (Game|Player|GetPlayerPawn 0)))
  (Variables|Default|SetPlayer _asbp_time_traveler)
  (Variables|Default|SetAnimInstance (Components|SkeletalMesh|GetAnimInstance (Variables|Character|GetMesh)))
  (Utilities|Array|Clear (Variables|Arrays|GetPatrolingLocations))
  (CallFunction|AddtoPatrolArray (Variables|Arrays|GetZoneArray6))
  (bind _returnvalue (CallFunction|GetRandomTargetPoint (Variables|Arrays|GetPatrolingLocations)))
  (Variables|AI|SetCurrentLocation _returnvalue)
  (Variables|/Script/Engine.PrimitiveComponent|SetbGenerateOverlapEvents (Variables|Default|GetAttackCollision) false)
  (Variables|AI|SetChanceToUpdateZone (Variables|AI|GetDefaultChanceToUpdateZone))
  ;[1 1 1] Bind hitbox damage delegates
  (for _array_element (Actor|GetComponentsByClass "/Script/GameOff2024.HitboxComponent")
    (switch Utilities|FlowControl|Switch|SwitchonEHitboxLocation (Variables|/Script/GameOff2024.HitboxComponent|GetLocation _array_element)
      (:EHL_Head
        (EventDispatchers|BindEventtoOnTakeHit _array_element (delegate Custom|Headshot)))
      (:EHL_Body
        (EventDispatchers|BindEventtoOnTakeHit _array_element (delegate Custom|Bodyshot)))
      (:EHL_Limb
        (EventDispatchers|BindEventtoOnTakeHit _array_element (delegate Custom|Limbshot))))))

(event EventTick
  (params (DeltaSeconds :type Float%20%28single-precision%29))
  (bind _patrolinglocations (Variables|Arrays|GetPatrolingLocations))
  ;[1 1 1] Handles The Patroling
  (if (not (Variables|AI|GetIsEntityRunning?))
    (if (not (Variables|AI|GetIsEntityChasingPlayer?))
      (if (not (Variables|AI|GetIsEntityInvestigating))
        (Variables|AI|SetIsEntityRunning? true)
        (Variables|/Script/Engine.CharacterMovementComponent|SetMaxWalkSpeed (Variables|Character|GetCharacterMovement) (Variables|Default|GetWalkSpeed))
        (if (Utilities|Array|IsValidIndex _patrolinglocations (Variables|AI|GetCurrentLocation))
          (AI|AIMoveTo self "0, 0, 0" (Utilities|Array|Get(acopy) _patrolinglocations (Variables|AI|GetCurrentLocation)) 5.0 false
            (:OnSuccess
              ;;[1 1 1] Cycles through the Array
              (Utilities|FlowControl|Delay (Math|Random|RandomFloatinRange 2.0 5.0))
              (if (not (or (Variables|AI|GetIsEntityChasingPlayer?) (Variables|AI|GetIsEntityInvestigating)))
                (Variables|AI|SetIsEntityRunning? false)
                (CallFunction|CyclingPatrolingArray (Variables|Arrays|GetPatrolingLocations))))
            (:OnFail
              (Development|PrintString "Patrol Failed")
              (Variables|AI|SetIsEntityRunning? false))))))))

(fn ConstructionScript)

(fn EntityAnimations
  (if (not (Variables|Default|GetIsEntityAnimRuningActive))
    (Variables|Default|SetIsEntityAnimRuningActive true)
    (Components|Animation|PlayAnimation (Variables|Character|GetMesh) 0 true)))

(fn CyclingPatrolingArray
  (params (TargetArray :type Array%20of%20Target%20Point%20Object%20References))
  (bind _returnvalue (Math|Random|RandomFloatinRange 0.0 1e+02))
  ;[1 1 1] Check if currently in player's zone
  (if (== (Variables|/Game/TimeTraval/BP_TimeTraveler.BP_TimeTraveler_C|GetCurrentZone (Variables|Default|GetPlayer)) (Variables|AI|GetCurrentZone))
    (Development|PrintString "Current Zone")
    ;[1 1 1] Select random target point and set current location
    (bind _returnvalue_2 (CallFunction|GetRandomTargetPoint TargetArray :!label _label))
    (Variables|AI|SetCurrentLocation _returnvalue_2)
    (Development|PrintString "Selected new random point")
    (else
      ;[1 1 1] Check if AI can enter safe zone if player is inside safe zone
      (if (and (== (Variables|/Game/TimeTraval/BP_TimeTraveler.BP_TimeTraveler_C|GetCurrentZone (Variables|Default|GetPlayer)) 1) (not (Variables|AI|GetCanEnterZone1)))
        (Development|PrintString "Player in safe zone, cannot enter")
        (goto _label)
        (else
          (Development|PrintString (Utilities|String|ToString(Float) _returnvalue))
          ;[1 1 1] Chance to update zone. Low = new zone, high = stay in old zone
          (if (>= _returnvalue (Variables|AI|GetChanceToUpdateZone))
            (Development|PrintString "Increasing chance")
            ;[1 1 1] Increase zone update chance if it's not already over 90%
            (if (<= (Variables|AI|GetChanceToUpdateZone) 9e+01)
              (Variables|AI|SetChanceToUpdateZone (+ (Variables|AI|GetChanceToUpdateZone) (Variables|AI|GetUpdateZoneRate)))
              (goto _label)
              (else
                (goto _label)))
            (else
              (Development|PrintString "Updating zone")
              (CallFunction|UpdateZone (Variables|/Game/TimeTraval/BP_TimeTraveler.BP_TimeTraveler_C|GetCurrentZone (Variables|Default|GetPlayer))))))))))

(fn GetRandomTargetPoint
  (params (TargetArray :type Array%20of%20Target%20Point%20Object%20References))
  (return (Math|Random|RandomInteger (Utilities|Array|Length TargetArray))))

(fn AddtoPatrolArray
  (params (Array :type Array%20of%20Target%20Point%20Object%20References))
  (for _array_element Array
    (Utilities|Array|AddUnique (Variables|Arrays|GetPatrolingLocations) _array_element))
  (return))

(fn UpdateZone
  (params (Zone :type Integer))
  ;[1 1 1] Clear patrol array and update zone to follow player
  (Variables|AI|SetChanceToUpdateZone (Variables|AI|GetDefaultChanceToUpdateZone))
  (Utilities|Array|Clear (Variables|Arrays|GetPatrolingLocations))
  (bind _output_get (Variables|AI|SetCurrentZone Zone))
  ;[1 1 1] Add new zone array to the patrol array
  (switch int _output_get
    (:1
      (CallFunction|AddtoPatrolArray (Variables|Arrays|GetZoneArray1)))
    (:2
      (CallFunction|AddtoPatrolArray (Variables|Arrays|GetZoneArray2)))
    (:3
      (CallFunction|AddtoPatrolArray (Variables|Arrays|GetZoneArray3)))
    (:4
      (CallFunction|AddtoPatrolArray (Variables|Arrays|GetZoneArray4)))
    (:5
      (CallFunction|AddtoPatrolArray (Variables|Arrays|GetZoneArray5)))
    (:6
      (CallFunction|AddtoPatrolArray (Variables|Arrays|GetZoneArray6)))
    (:7
      (CallFunction|AddtoPatrolArray (Variables|Arrays|GetZoneArray7)))
    (:8
      (CallFunction|AddtoPatrolArray (Variables|Arrays|GetZoneArray8))))
  ;[1 1 1] Select random target point and set current location
  (bind _returnvalue (CallFunction|GetRandomTargetPoint (Variables|Arrays|GetPatrolingLocations)))
  (Variables|AI|SetCurrentLocation _returnvalue))

(fn AttackPlayer
  (Animation|Montage|MontagePlay (Variables|Default|GetAnimInstance) "/Game/Blueprints/Enemy/Animations/Montages/AM_EntityAttack.AM_EntityAttack" 1.0 "MontageLength" 0.0 true))

(fn InitiateChase
  (Variables|AI|SetIsEntityChasingPlayer? true)
  (Variables|AI|SetIsEntityInvestigating false)
  (Variables|AI|SetIsEntityRunning? false)
  (Variables|/Script/Engine.CharacterMovementComponent|SetMaxWalkSpeed (Variables|Character|GetCharacterMovement) (Variables|Default|GetChaseSpeed)))

(fn StartDetection
  (Variables|Detection|SetDetectingPlayer true))

(fn DetectPlayer
  (Variables|Detection|SetDetection (+ (Variables|Detection|GetDetection) (Variables|Detection|GetDetectionRate))))

(fn StopDetection
  (Variables|Detection|SetDetectingPlayer false)
  (Development|PrintString "stop detection")
  (CallFunction|ResetAlertSound))

(fn SetDetectionRate
  (bind _player (Variables|Default|GetPlayer))
  (bind _charactermovement (Variables|/Script/Engine.Character|GetCharacterMovement _player))
  (if (AI|Components|NavMovement|IsCrouching _charactermovement)
    (Variables|Detection|SetDetectionRate 0.1)
    (elif (== (Variables|/Script/Engine.CharacterMovementComponent|GetMaxWalkSpeed _charactermovement) (Variables|/Script/GameOff2024.GameOff2024Character|GetMaxSprintSpeed _player))
      (Variables|Detection|SetDetectionRate 0.35)
      (else
        (Variables|Detection|SetDetectionRate 0.15)))))

(fn UpdateLastKnownLocation
  (bind _player (Variables|Default|GetPlayer))
  (bind _returnvalue (Transformation|GetActorLocation _player))
  (bind _outhit (Collision|LineTraceByChannel (Transformation|GetActorLocation _player) (Math|Vector|MakeVector (.x _returnvalue) (.y _returnvalue) (- (.z _returnvalue) 1e+03)) "TraceTypeQuery1" false (Utilities|Array|MakeArray _player) "ForDuration"))
  (Variables|Default|SetLastKnownLocation (.Location (Collision|BreakHitResult _outhit))))

(fn DamagePlayer
  (bind _player (Variables|Default|GetPlayer))
  (bind _output_get (Variables|/Script/GameOff2024.GameOff2024Character|SetCurrentHealth _player (Math|Integer|Clamp(Integer) (- (Variables|/Script/GameOff2024.GameOff2024Character|GetCurrentHealth _player) 35) 0 (Variables|/Script/GameOff2024.GameOff2024Character|GetMaxHealth _player))))
  (if (<= _output_get 0)
    (bind _asbp_time_traveler (Utilities|Casting|CastToBP_TimeTraveler (Game|Player|GetPlayerPawn 0)))
    (Default|Death _asbp_time_traveler)))