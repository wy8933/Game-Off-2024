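; BP_MusicSheet is a clue actor that registers when the time traveler has seen its music notes.
; While the player is inside its Box trigger, Tick runs a check, throttled by a half-second delay.
; The check uses a view-direction dot product and requires the Magnifier as active tool.
; On success it sets HasSeenMusicNotes on the player and disables its tick.
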(event OnComponentBeginOverlap(Box)
  (params (OverlappedComponent :type Primitive%20Component%20Object%20Reference) (OtherActor :type Actor%20Object%20Reference) (OtherComp :type Primitive%20Component%20Object%20Reference) (OtherBodyIndex :type Integer) (bFromSweep :type Boolean) (SweepResult :type Hit%20Result%20Structure%20%28by%20ref%29))
  (Utilities|Casting|CastToBP_TimeTraveler OtherActor)
  (Variables|Default|SetPlayerIsInStudio true))

(event OnComponentEndOverlap(Box)
  (params (OverlappedComponent :type Primitive%20Component%20Object%20Reference) (OtherActor :type Actor%20Object%20Reference) (OtherComp :type Primitive%20Component%20Object%20Reference) (OtherBodyIndex :type Integer))
  (Utilities|Casting|CastToBP_TimeTraveler OtherActor)
  (Variables|Default|SetPlayerIsInStudio false))

(event Custom|Check
  (bind _returnvalue (Game|Player|GetPlayerPawn 0))
  (bind _asbp_time_traveler (Utilities|Casting|CastToBP_TimeTraveler _returnvalue))
  (if (and (>= (* (Math|Vector|DotProduct (Math|Vector|GetForwardVector (Math|Rotator|FindLookatRotation (Transformation|GetActorLocation) (Transformation|GetActorLocation _returnvalue))) (Math|Vector|GetForwardVector (Pawn|GetControlRotation (Game|GetPlayerController 0) :!class /Script/Engine.Controller))) -1.0) 0.7) (== (Variables|/Script/GameOff2024.GameOff2024Character|GetCurrentActiveTool _asbp_time_traveler) (Variables|/Script/GameOff2024.GameOff2024Character|GetMagnifier _asbp_time_traveler)))
    (Development|PrintString "Look at is true")
    (Variables|/Game/TimeTraval/BP_TimeTraveler.BP_TimeTraveler_C|SetbHasSeenMusicNotes (Variables|Default|GetPlayer) true)
    (Development|PrintString "Saw music sheet")
    (Actor|Tick|SetActorTickEnabled false)
    (else
      (Development|PrintString "Look at is false"))))

(event EventBeginPlay
  (bind _asbp_time_traveler (Utilities|Casting|CastToBP_TimeTraveler (Game|Player|GetPlayerPawn 0)))
  (Variables|Default|SetPlayer _asbp_time_traveler))

(event Collision|EventActorBeginOverlap
  (params (OtherActor :type Actor%20Object%20Reference)))

(event EventTick
  (params (DeltaSeconds :type Float%20%28single-precision%29))
  (if (Variables|Default|GetPlayerIsInStudio)
    (if (not (Variables|Default|GetChecking))
      (Variables|Default|SetChecking true)
      (CallFunction|Check)
      (Utilities|FlowControl|Delay 0.5)
      (Variables|Default|SetChecking false))))

(fn ConstructionScript)