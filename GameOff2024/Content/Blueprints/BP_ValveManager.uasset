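; Valve puzzle manager that reveals a hidden water actor and key once every valve is in its correct state.
; The CheckValves event scans the Valves array and clears the AllCorrect flag if any valve is wrong.
; Success sets a Solved latch that skips later checks, while failure resets the flag for the next check.
; Debug prints report wrong valves and the solved state.
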(event Custom|CheckValves
  (if (not (Variables|Default|GetbSolved))
    (for _array_element (Variables|Default|GetValves)
      (if (not (Variables|/Game/Blueprints/Interactable/BP_PressureValve.BP_PressureValve_C|GetbCorrect _array_element))
        (Variables|Default|SetbAllCorrect false)
        (Development|PrintString "Not all valves are correct")))
    (if (Variables|Default|GetbAllCorrect)
      (Variables|Default|SetbSolved true)
      (Rendering|SetActorHiddenInGame (Variables|Default|GetWater) false)
      (Rendering|SetActorHiddenInGame (Variables|Default|GetKey) false)
      (Development|PrintString "All valves are correct")
      (else
        (Variables|Default|SetbAllCorrect true)))))

(event EventBeginPlay)

(event Collision|EventActorBeginOverlap
  (params (OtherActor :type Actor%20Object%20Reference)))

(event EventTick
  (params (DeltaSeconds :type Float%20%28single-precision%29)))

(fn ConstructionScript)