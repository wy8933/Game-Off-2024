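; Player pawn for a time-travel mechanic, with camera head bob and a key-triggered jump to the position of a player copy.
; Every tick, velocity selects an idle, walk or sprint camera shake to start on the player controller.
; Pressing T moves the pawn to PlayerCopy's transform, inverts that copy's ZDifference so the vertical offset flips, and prints the new transform.
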(event Custom|HeadBob
  (bind _returnvalue (Transformation|GetVelocity))
  (bind _returnvalue_2 (Game|GetPlayerController 0))
  (bind _returnvalue_3 (Math|Vector|VectorLength _returnvalue))
  ;[1 1 1] HeadBob
  (if (> _returnvalue_3 0.0)
    (if (<= _returnvalue_3 (Variables|Default|GetWalkSpeed))
      (Game|Feedback|ClientStartCameraShake _returnvalue_2 "/Game/FirstPerson/Blueprints/HeadBob/BP_HeadBob_Walk.BP_HeadBob_Walk_C" 1.0 "CameraLocal" "0, 0, 0")
      (else
        (Game|Feedback|ClientStartCameraShake _returnvalue_2 "/Game/FirstPerson/Blueprints/HeadBob/BP_HeadBob_Sprint.BP_HeadBob_Sprint_C" 1.0 "CameraLocal" "0, 0, 0")))
    (else
      (Game|Feedback|ClientStartCameraShake _returnvalue_2 "/Game/FirstPerson/Blueprints/HeadBob/BP_HeadBob_Idle.BP_HeadBob_Idle_C" 1.0 "CameraLocal" "0, 0, 0"))))

(event EventTick
  (params (DeltaSeconds :type Float%20%28single-precision%29))
  ;[1 1 1] HeadBob
  (CallFunction|HeadBob))

(event Input|KeyboardEvents|T
  (params (Key :type Key%20Structure :default "None"))
  (bind _playercopy (Variables|Default|GetPlayerCopy))
  (:Pressed
    (bind _playercopy_2 (Variables|Default|GetPlayerCopy)
      (:then
        (Transformation|SetActorTransform (Transformation|GetActorTransform _playercopy_2))
        (Variables|/Game/TimeTraval/BP_PlayerCopy.BP_PlayerCopy_C|SetZDifference _playercopy (* (Variables|/Game/TimeTraval/BP_PlayerCopy.BP_PlayerCopy_C|GetZDifference _playercopy) -1.0))
        (Development|PrintString (Utilities|String|ToString(Transform) (Transformation|GetActorTransform))))
      (:else))))

(fn ConstructionScript)