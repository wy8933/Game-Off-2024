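; BP_TimeTraveler is the first-person player character, with tool child actors, head bob, safe-code checking and death/respawn camera sequences.
; It swaps between a flickering lighter that sprinting extinguishes and a chargeable flashlight whose beam decays on timers.
; Flashlight charging and surface-traced footsteps report noise events scaled by charge level or gait, with debug spheres.
; Light raise/lower moves share MoveUp/MoveDown, resuming through integer Wait IDs dispatched by ReturnAfterWait.
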(event Custom|HeadBob
  (bind _returnvalue (Game|GetPlayerController 0))
  (bind _returnvalue_2 (Transformation|GetVelocity))
  (bind _returnvalue_3 (Math|Vector|VectorLength _returnvalue_2))
  ;[1 1 1] HeadBob
  (if (> _returnvalue_3 0.0)
    (if (<= _returnvalue_3 (Variables|Default|GetWalkSpeed))
      (Variables|Default|SetSprint false)
      (Game|Feedback|ClientStartCameraShake _returnvalue "/Game/FirstPerson/Blueprints/HeadBob/BP_HeadBob_Walk.BP_HeadBob_Walk_C" (* (Variables|Default|GetCameraShakeStrength) (Variables|Default|GetCameraShakeMultiplier)) "CameraLocal" "0, 0, 0")
      (else
        (Variables|Default|SetSprint true)
        (Game|Feedback|ClientStartCameraShake _returnvalue "/Game/FirstPerson/Blueprints/HeadBob/BP_HeadBob_Sprint.BP_HeadBob_Sprint_C" (* (Variables|Default|GetCameraShakeStrength) (Variables|Default|GetCameraShakeMultiplier)) "CameraLocal" "0, 0, 0")))
    (else
      (Game|Feedback|ClientStartCameraShake _returnvalue "/Game/FirstPerson/Blueprints/HeadBob/BP_HeadBob_Idle.BP_HeadBob_Idle_C" (* (Variables|Default|GetCameraShakeStrength) (Variables|Default|GetCameraShakeMultiplier)) "CameraLocal" "0, 0, 0"))))

(event Custom|Death
  ;[1 0.1979 0.1979] Death/Respawn
  (Rendering|SetVisibility (Variables|Default|GetFirstPersonCameraComponent) false false)
  (Input|DisableInput (Game|GetPlayerCharacter 0) (Game|GetPlayerController 0))
  (bind _returnvalue (Game|SpawnActorfromClass "/Game/Blueprints/LevelProgression/BP_CameraAnimationPlayer.BP_CameraAnimationPlayer_C" (Transformation|GetActorTransform (Game|Player|GetPlayerPawn 0)) "Undefined" "MultiplyWithRoot" 0 0))
  (Default|PlayDeathCameraAnimation _returnvalue)
  (Utilities|FlowControl|Delay 3.0)
  (Rendering|SetVisibility (Variables|Default|GetFlashlightSpotlight) false false)
  (bind _asgi_game (Utilities|Casting|CastToGI_Game (Game|GetGameInstance)))
  (bind _asbp_time_traveler (Utilities|Casting|CastToBP_TimeTraveler (Game|GetPlayerCharacter 0)))
  (Default|RespawnPlayer _asgi_game)
  (Transformation|SetActorTransform _returnvalue (Math|Transform|MakeTransform (.location (Variables|BP_TimeTraveler_C|GetSpawnPosition _asbp_time_traveler)) (.rotation (Transformation|GetActorTransform _asbp_time_traveler)) "1.000000,1.000000,1.000000"))
  (Default|PlaySpawnCameraAnimation _returnvalue)
  (Utilities|FlowControl|Delay 1.5)
  (Game|Player|SetViewTargetwithBlend (Game|GetPlayerController 0) self 1.0 "VTBlend_Cubic" 0.0 false)
  (Utilities|FlowControl|Delay 1.5)
  (Actor|DestroyActor _returnvalue)
  (Input|EnableInput (Game|GetPlayerCharacter 0) (Game|GetPlayerController 0))
  (Rendering|SetVisibility (Variables|Default|GetFirstPersonCameraComponent) true false))

(event Custom|Wait%201
  ;[0.1745 0.409 1] Light Sources
  ;;[1 1 1] Swap Light Source
  ;;;[1 1 1] Swap to Flashlight
  (Rendering|SetVisibility (Variables|Default|GetFlashlightMesh) true false)
  (if (> (Variables|Light|GetFlashlightChargeValue) 0)
    (Rendering|SetVisibility (Variables|Default|GetFlashlightSpotlight) true false))
  (CallFunction|MoveUp (Variables|Default|GetFlashlightMesh) 2))

(event Custom|Wait%203
  ;[0.1745 0.409 1] Light Sources
  ;;[1 1 1] Swap Light Source
  ;;;[1 1 1] Swap to Lighter
  (if (Variables|Default|GetIsSprinting)
    _
    (else
      (Rendering|SetVisibility (Variables|Default|GetLighterPointLight) true false)))
  (Rendering|SetVisibility (Variables|Default|GetLighterMesh) true false)
  (CallFunction|MoveUp (Variables|Default|GetLighterMesh) 4))

(event Custom|Wait%205
  ;[0.1745 0.409 1] Light Sources
  ;;[1 1 1] Pull Out / Put Away Light Source
  ;;;[1 1 1] Flashlight
  (Variables|Light|SetLightReady true))

(event Custom|Wait%206
  ;[0.1745 0.409 1] Light Sources
  ;;[1 1 1] Pull Out / Put Away Light Source
  ;;;[1 1 1] Flashlight
  (Rendering|SetVisibility (Variables|Default|GetFlashlightMesh) false true)
  (Variables|Light|SetLightReady true))

(event Custom|Wait%207
  ;[0.1745 0.409 1] Light Sources
  ;;[1 1 1] Pull Out / Put Away Light Source
  ;;;[1 1 1] Lighter
  (Variables|Light|SetLightReady true))

(event Custom|DecreaseFlashlightCharge
  (bind _flashlightspotlight (Variables|Default|GetFlashlightSpotlight))
  (bind _flashlightspotlight_2 (Variables|Default|GetFlashlightSpotlight))
  ;[0.1745 0.409 1] Light Sources
  ;;[1 1 1] Decrease Flashlight Charge
  (Rendering|Lighting|SetAttenuationRadius _flashlightspotlight (- (Variables|/Script/Engine.LocalLightComponent|GetAttenuationRadius _flashlightspotlight) 1e+03))
  (Rendering|Lighting|SetOuterConeAngle _flashlightspotlight_2 (- (Variables|/Script/Engine.SpotLightComponent|GetOuterConeAngle _flashlightspotlight_2) 5.0))
  (bind _result (Math|Integer|DecrementInt (Variables|Light|GetFlashlightChargeValue))
    (:%20%20
      (Variables|Light|SetFlashlightChargeValue _result)
      (if (> (Variables|Light|GetFlashlightChargeValue) 0)
        (if (Utilities|Time|IsValidTimerHandle (Variables|Light|GetFlashlightChargeTimer))
          (Utilities|Time|ClearandInvalidateTimerbyHandle (Variables|Light|GetFlashlightChargeTimer)))
        (bind _returnvalue (CallFunction|DetermineFlashlightChargeDuration))
        (bind _returnvalue_2 (Utilities|Time|SetTimerbyEvent (delegate Custom|DecreaseFlashlightCharge) _returnvalue))
        (Variables|Light|SetFlashlightChargeTimer _returnvalue_2)
        (else
          (Rendering|SetVisibility (Variables|Default|GetFlashlightSpotlight) false false))))))

(event Custom|Move%20Down
  (params (Component :type Scene%20Component%20Object%20Reference) (Wait :type Integer))
  (bind _relativelocation (Variables|/Script/Engine.SceneComponent|GetRelativeLocation Component))
  ;[0.1745 0.409 1] Light Sources
  ;;[1 1 1] Moving Lights
  (Components|MoveComponentTo Component (Math|Vector|MakeVector (.x _relativelocation) (.y _relativelocation) (- (.z _relativelocation) (Variables|Light|GetLightOffset))) (Variables|/Script/Engine.SceneComponent|GetRelativeRotation Component) true true 0.5 false)
  (CallFunction|ReturnAfterWait Wait))

(event Custom|Move%20Up
  (params (Component :type Scene%20Component%20Object%20Reference) (Wait :type Integer))
  (bind _relativelocation (Variables|/Script/Engine.SceneComponent|GetRelativeLocation Component))
  ;[0.1745 0.409 1] Light Sources
  ;;[1 1 1] Moving Lights
  (Components|MoveComponentTo Component (Math|Vector|MakeVector (.x _relativelocation) (.y _relativelocation) (+ (.z _relativelocation) (Variables|Light|GetLightOffset))) (Variables|/Script/Engine.SceneComponent|GetRelativeRotation Component) true true 0.5 false)
  (CallFunction|ReturnAfterWait Wait))

(event Custom|Safe%20Code
  (bind _safeactor (Variables|Default|GetSafeActor))
  ;[1 1 1] Safe Code
  (bind _result (Math|Integer|IncrementInt (Variables|Default|GetSafeCodeProgress))
    (:%20%20
      (bind _output_get (Variables|Default|SetSafeCodeProgress _result))
      (switch int _output_get
        (:1
          (if (== (Variables|Default|GetSafeCodeCurrentNumber) 0)
            (Development|PrintString "Correct")
            (else
              (Variables|Default|SetSafeCodeProgress 0))))
        (:2
          (if (== (Variables|Default|GetSafeCodeCurrentNumber) 4)
            (Development|PrintString "Correct")
            (else
              (Variables|Default|SetSafeCodeProgress 0))))
        (:3
          (if (== (Variables|Default|GetSafeCodeCurrentNumber) 5)
            (Development|PrintString "Correct")
            (else
              (Variables|Default|SetSafeCodeProgress 0))))
        (:4
          (if (== (Variables|Default|GetSafeCodeCurrentNumber) 1)
            (Utilities|IsValid _safeactor
              (:Is%20Valid
                (Default|OpenDoor _safeactor)
                (Development|PrintString "Correct")))
            (else
              (Variables|Default|SetSafeCodeProgress 0))))))))

(event Custom|Wait%204
  ;[0.1745 0.409 1] Light Sources
  ;;[1 1 1] Swap Light Source
  ;;;[1 1 1] Swap to Lighter
  (Rendering|SetVisibility (Variables|Default|GetFlashlightMesh) false true)
  (Variables|Light|SetLightReady true))

(event Custom|Wait%208
  ;[0.1745 0.409 1] Light Sources
  ;;[1 1 1] Pull Out / Put Away Light Source
  ;;;[1 1 1] Lighter
  (Rendering|SetVisibility (Variables|Default|GetLighterMesh) false true)
  (Variables|Light|SetLightReady true))

(event Custom|Wait%202
  ;[0.1745 0.409 1] Light Sources
  ;;[1 1 1] Swap Light Source
  ;;;[1 1 1] Swap to Flashlight
  (Rendering|SetVisibility (Variables|Default|GetLighterMesh) false true)
  (Variables|Light|SetLightReady true))

(event Input|EnhancedActionEvents|EnhancedInputActionIA_Move
  (params (ActionValue :type Vector%202D%20Structure) (ElapsedSeconds :type Float%20%28double-precision%29) (TriggeredSeconds :type Float%20%28double-precision%29) (InputAction :type Input%20Action%20Object%20Reference :default "/Game/FirstPerson/Input/Actions/IA_Move.IA_Move"))
  (|Footsteps))

(event Input|EnhancedActionEvents|EnhancedInputActionIA_ChargeLight
  (params (ActionValue :type Boolean) (ElapsedSeconds :type Float%20%28double-precision%29) (TriggeredSeconds :type Float%20%28double-precision%29) (InputAction :type Input%20Action%20Object%20Reference :default "/Game/FirstPerson/Input/Actions/IA_ChargeLight.IA_ChargeLight"))
  (bind _returnvalue (Transformation|GetActorLocation))
  (bind _returnvalue_2 (Transformation|GetActorLocation))
  (bind _returnvalue_3 (Transformation|GetActorLocation))
  (bind _returnvalue_4 (Transformation|GetActorLocation))
  (bind _flashlightspotlight (Variables|Default|GetFlashlightSpotlight))
  (bind _flashlightspotlight_2 (Variables|Default|GetFlashlightSpotlight))
  (bind _flashlightspotlight_3 (Variables|Default|GetFlashlightSpotlight))
  ;[0.1745 0.409 1] Light Sources
  ;;[1 1 1] Charge Flashlight
  (:Started
    (if (and (Variables|Light|GetLightToggle) (Variables|Light|GetLightReady))
      (if (and (Variables|Light|GetLightSourceIsFlashlight) (< (Variables|Light|GetFlashlightChargeValue) (Variables|Light|GetMaxFlashlightCharge)))
        (if (Utilities|Time|IsValidTimerHandle (Variables|Light|GetFlashlightChargeTimer))
          (Utilities|Time|ClearandInvalidateTimerbyHandle (Variables|Light|GetFlashlightChargeTimer)))
        (bind _result (Math|Integer|IncrementInt (Variables|Light|GetFlashlightChargeValue))
          (:%20%20
            (bind _output_get (Variables|Light|SetFlashlightChargeValue _result))
            (switch int _output_get
              (:1
                (Audio|SpawnSoundatLocation "/Game/Audio_Game/Audio_Content/SFX/Equips/MS_Equip_Lamp.MS_Equip_Lamp" _returnvalue "0, 0, 0" 1.0 1.0 0.0 0 0)
                (Class|AISenseHearing|ReportNoiseEvent _returnvalue_3 1.0 self 7e+02 "None")
                (Rendering|Debug|DrawDebugSphere _returnvalue_3 7e+02 12 "(R=0.109016,G=0.000000,B=1.000000,A=1.000000)" 1e+01)
                (Rendering|Lighting|SetAttenuationRadius _flashlightspotlight 2e+03)
                (Rendering|Lighting|SetOuterConeAngle _flashlightspotlight 2e+01)
                (Rendering|SetVisibility _flashlightspotlight true false))
              (:2
                (Audio|SpawnSoundatLocation "/Game/Audio_Game/Audio_Content/SFX/Equips/MS_Equip_Lamp.MS_Equip_Lamp" _returnvalue "0, 0, 0" 1.0 1.0 0.0 0 0)
                (Class|AISenseHearing|ReportNoiseEvent _returnvalue_4 1.0 self 1e+03 "None")
                (Rendering|Debug|DrawDebugSphere _returnvalue_4 1e+03 12 "(R=0.109016,G=0.000000,B=1.000000,A=1.000000)" 1e+01)
                (Rendering|Lighting|SetAttenuationRadius _flashlightspotlight_2 3e+03)
                (Rendering|Lighting|SetOuterConeAngle _flashlightspotlight_2 25.0))
              (:3
                (Audio|SpawnSoundatLocation "/Game/Audio_Game/Audio_Content/SFX/Equips/MS_Equip_Lamp.MS_Equip_Lamp" _returnvalue "0, 0, 0" 1.0 1.0 0.0 0 0)
                (Class|AISenseHearing|ReportNoiseEvent _returnvalue_2 1.0 self 1.5e+03 "None")
                (Rendering|Debug|DrawDebugSphere _returnvalue_2 1.5e+03 12 "(R=0.109016,G=0.000000,B=1.000000,A=1.000000)" 1e+01)
                (Rendering|Lighting|SetAttenuationRadius _flashlightspotlight_3 4e+03)
                (Rendering|Lighting|SetOuterConeAngle _flashlightspotlight_3 3e+01)))
            (bind _returnvalue_5 (CallFunction|DetermineFlashlightChargeDuration))
            (bind _returnvalue_6 (Utilities|Time|SetTimerbyEvent (delegate Custom|DecreaseFlashlightCharge) _returnvalue_5))
            (Variables|Light|SetFlashlightChargeTimer _returnvalue_6)
            (Components|Animation|PlayAnimation (Variables|Default|GetFlashlightMesh) "/Game/Assets/Environment/Models/FlashLight/lighter_Anim_Click_001.lighter_Anim_Click_001" false)))
        (else
          ;;[1 1 1] Reignite Lighter
          (if (not (Variables|Light|GetLightSourceIsFlashlight))
            (Rendering|SetVisibility (Variables|Default|GetLighterPointLight) true false)))))))

(event Input|EnhancedActionEvents|EnhancedInputActionIA_SwapLightSource
  (params (ActionValue :type Boolean) (ElapsedSeconds :type Float%20%28double-precision%29) (TriggeredSeconds :type Float%20%28double-precision%29) (InputAction :type Input%20Action%20Object%20Reference :default "/Game/FirstPerson/Input/Actions/IA_SwapLightSource.IA_SwapLightSource"))
  ;[0.1745 0.409 1] Light Sources
  ;;[1 1 1] Swap Light Source
  (:Started
    (if (Variables|Light|GetLightReady)
      (Variables|Light|SetLightReady false)
      (bind _output_get (Variables|Light|SetLightSourceIsFlashlight (not (Variables|Light|GetLightSourceIsFlashlight))))
      (if _output_get
        ;;;[1 1 1] Swap to Flashlight
        (if (Variables|Light|GetLightToggle)
          (CallFunction|MoveDown (Variables|Default|GetLighterMesh) 1)
          (else
            (Rendering|SetVisibility (Variables|Default|GetFlashlightMesh) true false)
            (if (> (Variables|Light|GetFlashlightChargeValue) 0)
              (Rendering|SetVisibility (Variables|Default|GetFlashlightSpotlight) true false))
            (CallFunction|MoveUp (Variables|Default|GetFlashlightMesh) 2)))
        (else
          ;;;[1 1 1] Swap to Lighter
          (if (Variables|Light|GetLightToggle)
            (CallFunction|MoveDown (Variables|Default|GetFlashlightMesh) 3)
            (else
              (if (Variables|Default|GetIsSprinting)
                _
                (else
                  (Rendering|SetVisibility (Variables|Default|GetLighterPointLight) true false)))
              (Rendering|SetVisibility (Variables|Default|GetLighterMesh) true false)
              (CallFunction|MoveUp (Variables|Default|GetLighterMesh) 4))))))))

(event Input|EnhancedActionEvents|EnhancedInputActionIA_Sprint
  (params (ActionValue :type Boolean) (ElapsedSeconds :type Float%20%28double-precision%29) (TriggeredSeconds :type Float%20%28double-precision%29) (InputAction :type Input%20Action%20Object%20Reference :default "/Game/FirstPerson/Input/Actions/IA_Sprint.IA_Sprint"))
  ;[0.1745 0.409 1] Light Sources
  ;;[1 1 1] Sprint extinguishing lighter
  (if (not (Variables|Default|GetbIsCrouched))
    (Rendering|SetVisibility (Variables|Default|GetLighterPointLight) false false)))

(event Input|EnhancedActionEvents|EnhancedInputActionIA_ToggleLight
  (params (ActionValue :type Boolean) (ElapsedSeconds :type Float%20%28double-precision%29) (TriggeredSeconds :type Float%20%28double-precision%29) (InputAction :type Input%20Action%20Object%20Reference :default "/Game/FirstPerson/Input/Actions/IA_ToggleLight.IA_ToggleLight"))
  ;[0.1745 0.409 1] Light Sources
  ;;[1 1 1] Pull Out / Put Away Light Source
  (:Started
    (if (Variables|Light|GetLightReady)
      (Variables|Light|SetLightReady false)
      (Variables|Light|SetLightToggle (not (Variables|Light|GetLightToggle)))
      (if (Variables|Light|GetLightSourceIsFlashlight)
        ;;;[1 1 1] Flashlight
        (if (Variables|Light|GetLightToggle)
          (Rendering|SetVisibility (Variables|Default|GetFlashlightMesh) true false)
          (if (> (Variables|Light|GetFlashlightChargeValue) 0)
            (Rendering|SetVisibility (Variables|Default|GetFlashlightSpotlight) true false))
          (CallFunction|MoveUp (Variables|Default|GetFlashlightMesh) 5)
          (else
            (CallFunction|MoveDown (Variables|Default|GetFlashlightMesh) 6)))
        (else
          ;;;[1 1 1] Lighter
          (if (Variables|Light|GetLightToggle)
            (Rendering|SetVisibility (Variables|Default|GetLighterMesh) true false)
            (if (Variables|Default|GetIsSprinting)
              _
              (else
                (Rendering|SetVisibility (Variables|Default|GetLighterPointLight) true false)))
            (CallFunction|MoveUp (Variables|Default|GetLighterMesh) 7)
            (else
              (CallFunction|MoveDown (Variables|Default|GetLighterMesh) 8))))))))

(event EventTick
  (params (DeltaSeconds :type Float%20%28single-precision%29))
  ;[1 1 1] Tick
  (CallFunction|HeadBob)
  (if (not (or (Variables|Light|GetLightSourceIsFlashlight) (Variables|Light|GetHasSetLightFlickerDelay)))
    (Variables|Light|SetHasSetLightFlickerDelay true)
    (Utilities|FlowControl|Delay (Math|Random|RandomFloatinRange 0.1 0.4))
    (Rendering|Lighting|SetAttenuationRadius (Variables|Default|GetLighterPointLight) (Math|Random|RandomFloatinRange 9e+02 1.6e+03))
    (Variables|Light|SetHasSetLightFlickerDelay false)))

(event EventBeginPlay
  ;[0.2889 1 0.3106] Initialize
  (Utilities|FlowControl|Sequence
    (:then_0
      (bind _save_settings (Class|BPIGameInstance|GetSettings(Message) (Game|GetGameInstance)))
      (Variables|Default|SetCameraShakeMultiplier (Variables|/Game/SaveGames/SV_Settings.SV_Settings_C|GetCameraShakeMultiplier _save_settings))
      ;;[1 1 1] Deactivate Tools
      (bind _asbottle_tool_actor (Utilities|Casting|CastToBottleToolActor (Variables|/Script/Engine.ChildActorComponent|GetChildActor (Variables|Default|GetBP_BottleToolActor))))
      (bind _output_get (Variables|Default|SetBottle _asbottle_tool_actor))
      (Class|ToolActor|SetActive _output_get false)
      (bind _asmagnifier_tool_actor (Utilities|Casting|CastToMagnifierToolActor (Variables|/Script/Engine.ChildActorComponent|GetChildActor (Variables|Default|GetBP_MagnifierToolActor))))
      (bind _output_get_2 (Variables|Default|SetMagnifier _asmagnifier_tool_actor))
      (Class|ToolActor|SetActive _output_get_2 false)
      (bind _asbp_gun_tool_actor (Utilities|Casting|CastToBP_GunToolActor (Variables|/Script/Engine.ChildActorComponent|GetChildActor (Variables|Default|GetBP_GunToolActor))))
      (bind _output_get_3 (Variables|Default|SetGun _asbp_gun_tool_actor))
      (Class|ToolActor|SetActive _output_get_3 false))
    (:then_1
      (bind _returnvalue (Actor|GetActorOfClass "/Script/Engine.PlayerStart"))
      (Variables|Default|SetSpawnPosition (Transformation|GetActorTransform _returnvalue))
      ;;[0.07036 0.1683 0.4072] Move lighter down since it's inactive
      (CallFunction|MoveDown (Variables|Default|GetLighterMesh))
      (bind _returnvalue_2 (Actor|GetActorOfClass "/Game/Blueprints/BP_Safe.BP_Safe_C"))
      (Variables|Default|SetSafeActor _returnvalue_2))))

(event Input|KeyboardEvents|9
  (params (Key :type Key%20Structure :default "None"))
  (:Pressed
    (Utilities|Casting|CastToBottlesHUDWidget (HUD|GetHUD (Game|GetPlayerController 0)))))

(event Input|KeyboardEvents|T
  (params (Key :type Key%20Structure :default "None"))
  ;[1 1 1] Set the player's transform to the clone, and revert the z difference the clone
  (:Pressed
    (Variables|Default|GetPlayerCopy
      (:then
        (Transformation|SetActorTransform (Transformation|GetActorTransform))
        (Variables|/Game/TimeTraval/BP_PlayerClone.BP_PlayerClone_C|SetZDifference (Variables|Default|GetPlayerCopy) 0.0))
      (:else))))

(fn ConstructionScript)

(fn DetermineFlashlightChargeDuration
  (return (Math|Conversions|ToFloat(Integer) (* (Variables|Light|GetFlashlightChargeValue) 5))))

(fn ReturnAfterWait
  (params (Wait :type Integer))
  (switch int Wait
    (:1
      (CallFunction|Wait1))
    (:2
      (CallFunction|Wait2))
    (:3
      (CallFunction|Wait3))
    (:4
      (CallFunction|Wait4))
    (:5
      (CallFunction|Wait5))
    (:6
      (CallFunction|Wait6))
    (:7
      (CallFunction|Wait7))
    (:8
      (CallFunction|Wait8))))

(event Custom|Reset%20Footstep
  (bind _returnvalue (Transformation|GetActorLocation))
  (bind _returnvalue_2 (Transformation|GetActorLocation))
  (bind _returnvalue_3 (Transformation|GetActorLocation))
  (Utilities|FlowControl|DoOnce false) ; enters at Reset
)