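; BP_PlayerClone is a copy of the time-traveling player that shadows them at a height offset.
; BeginPlay caches the player character as BP_TimeTraveler.
; Each Tick it takes the player's transform, adding ZDifference to the Z location.
; Its Camera copies the relative transform of the player's MagnifyGlasses component, except rotation pitch, giving a matching viewpoint at the offset height.
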(event EventBeginPlay
  ;[1 1 1] Init the Player
  (bind _asbp_time_traveler (Utilities|Casting|CastToBP_TimeTraveler (Game|GetPlayerCharacter 0)))
  (Variables|Default|SetPlayer _asbp_time_traveler))

(event Collision|EventActorBeginOverlap
  (params (OtherActor :type Actor%20Object%20Reference)))

(event EventTick
  (params (DeltaSeconds :type Float%20%28single-precision%29))
  (bind _returnvalue (Game|GetPlayerCharacter 0))
  (bind _player (Variables|Default|GetPlayer))
  (bind _returnvalue_2 (Transformation|GetActorTransform _returnvalue))
  (bind _magnifyglasses (Variables|/Game/TimeTraval/BP_TimeTraveler.BP_TimeTraveler_C|GetMagnifyGlasses _player))
  (bind _returnvalue_3 (Transformation|GetRelativeTransform _magnifyglasses))
  ;[1 1 1] Set the transform of player copy reletive to player's x and y coordinates, and apply z coordinate with offsets
  (Transformation|SetActorTransform (Math|Transform|MakeTransform (Math|Vector|MakeVector (.x (.location _returnvalue_2)) (.y (.location _returnvalue_2)) (+ (.z (.location _returnvalue_2)) (Variables|Default|GetZDifference))) (.rotation _returnvalue_2) (.scale _returnvalue_2)))
  ;[1 1 1] Make sure player copy's camera's transform is the same as the player
  (Transformation|SetRelativeTransform (Variables|Default|GetCamera) (Math|Transform|MakeTransform (.location _returnvalue_3) (Math|Rotator|MakeRotator (.roll (.rotation _returnvalue_3)) 0.0 (.yaw (.rotation _returnvalue_3))) (.scale _returnvalue_3)) false false))

(fn ConstructionScript)